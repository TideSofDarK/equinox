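; BP_Ghost is a ghost character whose mesh is partly physics-simulated.
; On BeginPlay it loops over six named bones and enables physics simulation on each one and the bodies below it.
; Each pass sets full physics blend weight only from a hard-coded Bone_010 down, not from the current bone.
; AI chase logic toward the player pawn is present but unconnected, so it never runs.
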(event `self.ReceiveBeginPlay`
  (`parent.ReceiveBeginPlay`)
  (for _array_element (`|MakeArray` "Bone_004" "Bone_006" "Bone_008" "Bone_010" "Bone_012" "Bone_014" :!type "Name")
    (`SkeletalMeshComponent.SetAllBodiesBelowSimulatePhysics` (`self.Mesh`) _array_element true true)
    (`SkeletalMeshComponent.SetAllBodiesBelowPhysicsBlendWeight` (`self.Mesh`) "Bone_010" 1.0 false true)))

(fn `UserConstructionScript`
  (`parent.UserConstructionScript`))