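; BP_Zombie is a zombie character that plays an attached hurt sound on damage while alive and ragdolls on death.
; EnableAI_Event spawns and possesses an AI controller if none is valid.
; Die switches the mesh to full physics simulation and detaches the controller.
; SpawnGib hides a listed bone and simulates it on a duplicate skeletal mesh, but its only call here is disconnected, as is a timeline-driven ragdoll blend.
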(event `self.ReceiveBeginPlay`)

(event `EnableAI_Event`
  (`/Engine/EditorBlueprintResources/StandardMacros.IsValid` (`AIBlueprintHelperLibrary.GetAIController` self)
    (:`Is Not Valid`
      (bind _returnvalue (`|SpawnActorFromClass` (`self.AIControllerClass`) (`KismetMathLibrary.MakeTransform` (0.0 0.0 0.0)) "Undefined" "OverrideRootScale" null null))
      (`Controller.Possess` _returnvalue self))))

(event `self.ReceiveAnyDamage`
  (params (Damage :type "Float (single-precision)") (DamageType :type "DamageType Object Reference") (InstigatedBy :type "Controller Object Reference") (DamageCauser :type "Actor Object Reference"))
  (if (not (`self.bIsDead`))
    (`GameplayStatics.SpawnSoundAttached` "/Game/FD10/Characters/Zombie_01/Audio/A_Zombie003_Hurt_A_Cue.A_Zombie003_Hurt_A_Cue" (`self.Mesh`) "Base-HumanHead" (0.0 0.0 0.0) (struct) "KeepRelativeOffset" false 1.0 1.0 0.0 null null)))

(event `self.ReceiveTick`
  (params (DeltaSeconds :type "Float (single-precision)")))

(event `self.Die`
  (`PrimitiveComponent.SetSimulatePhysics` (`self.Mesh`) true)
  (`SkeletalMeshComponent.SetAllBodiesSimulatePhysics` (`self.Mesh`) true)
  (`SkeletalMeshComponent.SetAllBodiesPhysicsBlendWeight` (`self.Mesh`) 1.0 false)
  (`self.DetachFromControllerPendingDestroy`))

(fn `Die2`)

(fn `SpawnGib`
  (locals (CachedGibName :type Name) (CachedGib :type "SkeletalMeshComponent Object Reference"))
  (if (> (`KismetArrayLibrary.Array_Length` (`self.GibNames`)) 0)
    (set `local.CachedGibName` (`|GetArrayItem` (`self.GibNames`)))
    (`KismetArrayLibrary.Array_Remove` (`self.GibNames`))
    (`SkinnedMeshComponent.HideBoneByName` (`self.Mesh`) (`local.CachedGibName`) "PBO_Term")
    (bind _returnvalue (`AddComponent|NODE_AddSkeletalMeshComponent-0` :`RelativeTransform` (`SceneComponent.GetRelativeTransform` (`self.Mesh`))))
    (bind _output_get (set `local.CachedGib` _returnvalue))
    (`SkinnedMeshComponent.SetSkinnedAssetAndUpdate` _output_get (`SkinnedMeshComponent.SkeletalMesh` (`self.Mesh`)) true)
    (`PrimitiveComponent.SetCollisionEnabled` (`local.CachedGib`) "PhysicsOnly")
    (`SkinnedMeshComponent.SetPhysicsAsset` (`local.CachedGib`) (`SkeletalMesh.PhysicsAsset` (`SkinnedMeshComponent.SkeletalMesh` (`self.Mesh`))) false)
    (`SkeletalMeshComponent.SetAllBodiesBelowSimulatePhysics` (`local.CachedGib`) (`local.CachedGibName`) true true)
    (`SkeletalMeshComponent.BreakConstraint` (`local.CachedGib`) (50.0 50.0 50.0) (0.0 0.0 0.0) (`local.CachedGibName`))))

(fn `UserConstructionScript`)