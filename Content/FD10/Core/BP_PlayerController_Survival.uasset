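; Player controller for the survival mode that manages inventory and stash item grids and opens their UI.
; On BeginPlay it adds the interact-target widget, spawns starting items into the inventory and uses Game and UI input.
; It creates pickup, inventory, stash and examination widgets, pausing during pickups and binding close callbacks.
; Free-slot search functions are unfinished stubs; F10 and F12 provide widget-count and garbage-collection debugging.
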(event `Key|F10` :paused true
  (params (Key :type "Key Structure"))
  (:`Pressed`
    (bind _foundwidgets (`WidgetBlueprintLibrary.GetAllWidgetsOfClass` "/Game/FD10/Widgets/Inventory/WBP_Item.WBP_Item_C" false))
    (`KismetSystemLibrary.PrintString` (`KismetStringLibrary.Conv_IntToString` (`KismetArrayLibrary.Array_Length` _foundwidgets)))
    (bind _foundwidgets_2 (`WidgetBlueprintLibrary.GetAllWidgetsOfClass` "/Game/FD10/Widgets/WBP_CaptureBox.WBP_CaptureBox_C" false))
    (`KismetSystemLibrary.PrintString` (`KismetStringLibrary.Conv_IntToString` (`KismetArrayLibrary.Array_Length` _foundwidgets_2)))
    (bind _foundwidgets_3 (`WidgetBlueprintLibrary.GetAllWidgetsOfClass` "/Game/FD10/Widgets/Inventory/WBP_ExamineTarget.WBP_ExamineTarget_C" false))
    (`KismetSystemLibrary.PrintString` (`KismetStringLibrary.Conv_IntToString` (`KismetArrayLibrary.Array_Length` _foundwidgets_3)))
    (bind _foundwidgets_4 (`WidgetBlueprintLibrary.GetAllWidgetsOfClass` "/Game/FD10/Widgets/Inventory/WBP_ItemExamination.WBP_ItemExamination_C" false))
    (`KismetSystemLibrary.PrintString` (`KismetStringLibrary.Conv_IntToString` (`KismetArrayLibrary.Array_Length` _foundwidgets_4)))))

(event `Key|F12` :paused true
  (params (Key :type "Key Structure"))
  (:`Pressed`
    (`KismetSystemLibrary.CollectGarbage`)))

(event `LoadItems_Event`
  (bind _returnvalue (`self.SpawnPickedItem` "/Game/FD10/Items/Weapons/Sigismund/BP_Sigismund.BP_Sigismund_C"))
  (`self.AddItemToInventory` _returnvalue (make `IntVector` 0))
  (bind _returnvalue_2 (`self.SpawnPickedItem` "/Game/FD10/Items/Weapons/Sigismund/BP_Sigismund_Ammo.BP_Sigismund_Ammo_C"))
  (`self.AddItemToInventory` _returnvalue_2 (make `IntVector` 1))
  (set `/Game/FD10/Core/Survival/Items/BP_Item_Survival.StackCount` 15 _returnvalue_2))

(event `self.ReceiveBeginPlay`
  (bind _returnvalue (`|CreateWidget` "/Game/FD10/Widgets/WBP_InteractTarget.WBP_InteractTarget_C" self))
  (`UserWidget.AddToViewport` _returnvalue 0)
  (`self.LoadItems_Event`)
  (`WidgetBlueprintLibrary.SetInputMode_GameAndUIEx` self null))

(event `OnItemPickup_Event`
  (params (Item :type "/Game/FD10/Core/Survival/Items/BP_Item_Survival Object Reference"))
  (`GameplayStatics.SetGamePaused` true)
  (bind _returnvalue (`|CreateWidget` "/Game/FD10/Widgets/ItemPickup/WBP_ItemPickup.WBP_ItemPickup_C" self Item))
  (`UserWidget.AddToPlayerScreen` _returnvalue 0)
  (add `/Game/FD10/Widgets/ItemPickup/WBP_ItemPickup.ItemPickupED` _returnvalue (delegate `OnItemPickupClosed_Event`)))

(event `OnItemPickupClosed_Event`
  (`GameplayStatics.SetGamePaused` false))

(event `self.ReceiveTick`
  (params (DeltaSeconds :type "Float (single-precision)")))

(event `InputAction|Inventory`
  (params (Key :type "Key Structure"))
  (:`Pressed`
    (`self.OpenInventory_Event` null)))

(event `OpenInventory_Event`
  (params (PickedItem :type "/Game/FD10/Core/Survival/Items/BP_Item_Survival Object Reference"))
  (bind _returnvalue (`|CreateWidget` "/Game/FD10/Widgets/Inventory/WBP_Inventory.WBP_Inventory_C" self PickedItem))
  (`UserWidget.AddToPlayerScreen` _returnvalue 0))

(fn `AddItemToInventory`
  (params (Item :type "/Game/FD10/Core/Survival/Items/BP_Item_Survival Object Reference") (Slot :type "IntVector Structure"))
  (`BlueprintMapLibrary.Map_Add` (`self.InventoryGrid`) Slot Item))

(fn `AddItemToStash`
  (params (Item :type "/Game/FD10/Core/Survival/Items/BP_Item_Survival Object Reference") (Slot :type "IntVector Structure"))
  (`BlueprintMapLibrary.Map_Add` (`self.StashGrid`) Slot Item))

(fn `FindFreeInventorySlot`
  (params (ItemClass :type "/Game/FD10/Core/Survival/Items/BP_Item_Survival Class Reference"))
  (returns (bFound :type Boolean) (Slot :type "IntVector Structure"))
  (bind (_inventorysize_x _inventorysize_y) (break `IntVector` (`self.InventorySize`)))
  (for _ (range _inventorysize_y)
    (for _ (range _inventorysize_x)
      _)))

(fn `IsInventoryQuadFree`
  (params (Size :type "IntVector Structure") (Slot :type "IntVector Structure")))

(fn `OpenItemExaminationWithCloseCallback`
  (params (Item :type "/Game/FD10/Core/Survival/Items/BP_Item_Survival Object Reference") (Event :type "Delegate (by ref)"))
  (bind _returnvalue (`|CreateWidget` "/Game/FD10/Widgets/Inventory/WBP_ItemExamination.WBP_ItemExamination_C" self Item))
  (`UserWidget.AddToPlayerScreen` _returnvalue 0)
  (add `/Game/FD10/Widgets/Inventory/WBP_ItemExamination.CloseED` _returnvalue Event)
  (`Widget.SetUserFocus` _returnvalue self)
  (return))

(fn `OpenStashWithCloseCallback`
  (params (Event :type "Delegate (by ref)"))
  (bind _returnvalue (`|CreateWidget` "/Game/FD10/Widgets/Inventory/WBP_Stash.WBP_Stash_C" self null))
  (`UserWidget.AddToPlayerScreen` _returnvalue 0)
  (add `/Game/FD10/Widgets/Inventory/WBP_Stash.StashED` _returnvalue Event)
  (return))

(fn `SpawnPickedItem`
  (params (ItemClass :type "/Game/FD10/Core/Survival/Items/BP_Item_Survival Class Reference"))
  (returns (ReturnValue :type "/Game/FD10/Core/Survival/Items/BP_Item_Survival Object Reference"))
  (bind _returnvalue (`GameplayStatics.GetPlayerPawn` 0))
  (bind _returnvalue_2 (`|SpawnActorFromClass` ItemClass (`KismetMathLibrary.MakeTransform` (0.0 0.0 0.0)) "AlwaysSpawn" "OverrideRootScale" null 1 null))
  (`/Engine/EditorBlueprintResources/StandardMacros.IsValid` _returnvalue
    (:`Is Valid`
      (`self.SetOwner` _returnvalue_2 _returnvalue))
    (:`Is Not Valid`
      _))
  (`/Game/FD10/Core/Survival/Items/BP_Item_Survival.OnPostPickup_Event` _returnvalue_2)
  (return _returnvalue_2))

(fn `UserConstructionScript`)