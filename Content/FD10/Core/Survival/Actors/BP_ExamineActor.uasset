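; Interactable examine point for the survival game that shows a sequence of typed text lines from its own view.
; On interaction it pauses the game and music, plays a bell, switches view target and input mode, and optionally hides the player.
; Primary input skips typing or advances the HUD examine widget, restoring everything after the last line.
; Separate events toggle camera aspect-ratio constraint for black bars, but nothing here calls them.
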(event `PrepareBlackBoxes_Event`
  (bind _aspectratio (`/Game/FD10/Core/Survival/BPFL_SurvivalUtilities.GetScreenAspectRatio`))
  (set `self.CachedAspectRatio` _aspectratio)
  (`CameraComponent.SetConstraintAspectRatio` (`self.Camera`) true))

(event `RevertBlackBoxes_Event`
  (`CameraComponent.SetConstraintAspectRatio` (`self.Camera`) false)
  (bind _aspectratio (`/Game/FD10/Core/Survival/BPFL_SurvivalUtilities.GetScreenAspectRatio`))
  (`CameraComponent.SetAspectRatio` (`self.Camera`) _aspectratio))

(event `AdvanceExamineText_Event`
  (bind _examinewidget (`/Game/FD10/Core/Survival/HUD_Survival.ExamineWidget` (`/Game/FD10/Core/Survival/BPFL_SurvivalUtilities.GetSurvivalHud`)))
  (if (`/Game/FD10/Widgets/WBP_Examine.bIsTyping` _examinewidget)
    (`/Game/FD10/Widgets/WBP_Examine.ForceStopTyping_Event` _examinewidget)
    (elif (>= (`self.TextIndex`) (`KismetArrayLibrary.Array_Length` (`self.ExamineTexts`)))
      (`self.OnExamineEnd_Event`)
      (else
        (`/Game/FD10/Widgets/WBP_Examine.SetTextForTyping` (`/Game/FD10/Core/Survival/HUD_Survival.ExamineWidget` (`/Game/FD10/Core/Survival/BPFL_SurvivalUtilities.GetSurvivalHud`)) (`|GetArrayItem` (`self.ExamineTexts`) (`self.TextIndex`)))
        (`/Engine/EditorBlueprintResources/StandardMacros.IncrementInt` (`self.TextIndex`))))))

(event `InputAction|Primary` :paused true
  (params (Key :type "Key Structure"))
  (:`Pressed`
    (`self.AdvanceExamineText_Event`)))

(event `self.ReceiveBeginPlay`
  (`parent.ReceiveBeginPlay`)
  (add `self.OnInteracted` (delegate `OnExamined_Event`)))

(event `OnExamined_Event`
  (bind _survivalplayercontroller (`/Game/FD10/Core/Survival/BPFL_SurvivalUtilities.GetSurvivalPlayerController`))
  (`self.AdvanceExamineText_Event`)
  (set `self.CachedViewTarget` (`Controller.GetViewTarget` (`GameplayStatics.GetPlayerController` 0)))
  (`PlayerController.SetViewTargetWithBlend` (`GameplayStatics.GetPlayerController` 0) self 0.0 "VTBlend_Linear" 0.0 false)
  (`/Game/FD10/Core/Survival/BP_SurvivalPlayerController.SetSurvivalInputMode_Event` _survivalplayercontroller "NewEnumerator1")
  (`self.EnableInput` _survivalplayercontroller)
  (`GameplayStatics.SetGamePaused` true)
  (`GameplayStatics.PlaySound2D` "/Game/FD10/Audio/Effects/A_Horror_Bell.A_Horror_Bell" 1.0 1.0 0.0 null null)
  (`/Game/FD10/Core/Survival/BP_SurvivalPlayerState.SetBGMPaused` (`/Game/FD10/Core/Survival/BPFL_SurvivalUtilities.GetSurvivalPlayerState`) true 0.0)
  (if (`self.bHidePlayer`)
    (`/Game/FD10/Core/Survival/Characters/BP_SurvivalCharacterBase.SetCharacterVisibility` (`/Game/FD10/Core/Survival/BPFL_SurvivalUtilities.GetSurvivalPlayerPawn`) false)))

(event `OnExamineEnd_Event`
  (bind _survivalplayercontroller (`/Game/FD10/Core/Survival/BPFL_SurvivalUtilities.GetSurvivalPlayerController`))
  (`PlayerController.SetViewTargetWithBlend` (`GameplayStatics.GetPlayerController` 0) (`self.CachedViewTarget`) 0.0 "VTBlend_Linear" 0.0 false)
  (`/Game/FD10/Core/Survival/BP_SurvivalPlayerController.SetSurvivalInputMode_Event` _survivalplayercontroller "NewEnumerator0")
  (`self.DisableInput` _survivalplayercontroller)
  (set `self.TextIndex` 0)
  (`/Game/FD10/Widgets/WBP_Examine.SetTextForTyping` (`/Game/FD10/Core/Survival/HUD_Survival.ExamineWidget` (`/Game/FD10/Core/Survival/BPFL_SurvivalUtilities.GetSurvivalHud`)) "")
  (`GameplayStatics.SetGamePaused` false)
  (`/Game/FD10/Core/Survival/BP_SurvivalPlayerState.SetBGMPaused` (`/Game/FD10/Core/Survival/BPFL_SurvivalUtilities.GetSurvivalPlayerState`) false 1.0)
  (if (`self.bHidePlayer`)
    (`/Game/FD10/Core/Survival/Characters/BP_SurvivalCharacterBase.SetCharacterVisibility` (`/Game/FD10/Core/Survival/BPFL_SurvivalUtilities.GetSurvivalPlayerPawn`) true)))

(fn `UserConstructionScript`
  (`parent.UserConstructionScript`))