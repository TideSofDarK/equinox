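; BP_Painting is an examinable painting actor for the survival game, built on a parent class that supplies the examine events.
; The construction script applies a configurable static mesh and puts the artwork material in slot 1, so instances can show different paintings.
; On examine, the CameraZoom timeline slides the actor's own camera along its relative X axis.
; The timeline is set tickable when paused, so the zoom keeps playing while the game is paused.
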(event `self.OnExamined_Event`
  (bind (_relativelocation_x _relativelocation_y _relativelocation_z) (`KismetMathLibrary.BreakVector` (`SceneComponent.RelativeLocation` (`self.Camera`))))
  (`parent.OnExamined_Event`)
  (bind (_direction _x) (`Timeline|CameraZoom` :!via `PlayFromStart`)
    (:`Update`
      (`SceneComponent.K2_SetRelativeLocation` (`self.Camera`) (`KismetMathLibrary.MakeVector` _x _relativelocation_y _relativelocation_z) false false))))

(event `self.OnExamineEnd_Event`
  (`parent.OnExamineEnd_Event`))

(event `self.ReceiveBeginPlay`
  (`parent.ReceiveBeginPlay`)
  (`ActorComponent.SetTickableWhenPaused` (`self.CameraZoom`) true))

(fn `UserConstructionScript`
  (`StaticMeshComponent.SetStaticMesh` (`self.StaticMesh`) (`self.PaintingStaticMesh`))
  (`PrimitiveComponent.SetMaterial` (`self.StaticMesh`) 1 (`self.ArtMaterial`))
  (`parent.UserConstructionScript`))