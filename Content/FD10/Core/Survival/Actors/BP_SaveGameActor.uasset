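; BP_SaveGameActor is an interactable world actor that serves as a save point in the survival game.
; On BeginPlay it binds its interaction event to a save handler.
; The handler captures a save screenshot via the player state, collapses the HUD, waits a zero-length delay, then pauses the game and opens the save game screen through the player controller.
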(event `self.ReceiveBeginPlay`
  (`parent.ReceiveBeginPlay`)
  (add `self.OnInteracted` (delegate `OnSaveGame_Event`)))

(event `OnSaveGame_Event`
  (`/Game/FD10/Core/Survival/BP_SurvivalPlayerState.CaptureSaveGameScreenshot` (`/Game/FD10/Core/Survival/BPFL_SurvivalUtilities.GetSurvivalPlayerState`))
  (`/Game/FD10/Core/Survival/HUD_Survival.SetGeneralHUDVisibility` (`/Game/FD10/Core/Survival/BPFL_SurvivalUtilities.GetSurvivalHud`) "Collapsed")
  (`KismetSystemLibrary.Delay` 0.0)
  (`GameplayStatics.SetGamePaused` true)
  (`/Game/FD10/Core/Survival/BP_SurvivalPlayerController.OpenSaveGameScreen` (`/Game/FD10/Core/Survival/BPFL_SurvivalUtilities.GetSurvivalPlayerController`)))

(fn `UserConstructionScript`
  (`parent.UserConstructionScript`))