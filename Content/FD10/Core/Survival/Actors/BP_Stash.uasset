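; BP_Stash is an interactable stash locker whose door swings open to give the player access to the stash.
; Interaction fires a FlipFlop: opening plays a creak and pauses the game, while a pause-tickable timeline rotates the door's yaw.
; When opening finishes, the survival player controller opens the stash with a close callback.
; The alternate toggle unpauses and reverses the door faster; each finished swing toggles interactable availability.
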(event `self.ReceiveBeginPlay`
  (add `/Game/FD10/Core/Survival/Components/BP_InteractableComponent.InteractableED` (`self.BP_InteractableComponent`) (delegate `ToggleDoor`))
  (`ActorComponent.SetTickableWhenPaused` (`self.DoorTimeline`) true))

(event `ToggleDoor`
  (bind _doortimeline (`self.DoorTimeline`))
  (`/Engine/EditorBlueprintResources/StandardMacros.FlipFlop`
    (:`A`
      (`TimelineComponent.SetPlayRate` _doortimeline 1.0)
      (`GameplayStatics.PlaySound2D` "/Game/FD10/Audio/StarterContent/A_LockerCreek_Cue.A_LockerCreek_Cue" 1.0 1.0 0.0 null null)
      (`GameplayStatics.SetGamePaused` true)
      (bind (_direction _z) (`Timeline|DoorTimeline` :!via `PlayFromStart` :!label _label)
        (:`Update`
          (`SceneComponent.K2_SetRelativeRotation` (`self.Scene`) (`KismetMathLibrary.MakeRotator` 0.0 0.0 _z) false false))
        (:`Finished`
          (`/Game/FD10/Core/Survival/Components/BP_InteractableComponent.ToggleAvailability_Event` (`self.BP_InteractableComponent`))
          (switch `ETimelineDirection` _direction
            (:`Forward`
              (bind _asbp_survival_player_controller (cast `/Game/FD10/Core/Survival/BP_SurvivalPlayerController` (`GameplayStatics.GetPlayerController` 0)))
              (`/Game/FD10/Core/Survival/BP_SurvivalPlayerController.OpenStashWithCloseCallback` _asbp_survival_player_controller (`|CreateDelegate` :!event `ToggleDoor`)))))))
    (:`B`
      (`TimelineComponent.SetPlayRate` _doortimeline 3.0)
      (`GameplayStatics.SetGamePaused` false)
      (goto _label :!via `ReverseFromEnd`))))

(fn `UserConstructionScript`)