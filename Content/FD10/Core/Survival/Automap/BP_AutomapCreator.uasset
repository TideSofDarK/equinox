(event `self.ReceiveBeginPlay`
  (bind _returnvalue (`LayersBlueprintLibrary.GetActors` (make `ActorLayer` "Automap")))
  (for _array_element _returnvalue
    (`self.K2_DestroyActor` _array_element)))

(event `/Game/FD10/Core/Survival/Levels/BPI_LevelBuilder.Build`
  (params (LevelManifest :type "/Game/FD10/Core/Survival/Levels/BP_LevelManifest Object Reference"))
  (`self.CreateTextureTarget`)
  (`self.CreateAutomapTexture`)
  (set `/Game/FD10/Core/Survival/Levels/BP_LevelManifest.AutomapTexture` (`self.AutomapTexture`) LevelManifest))

(fn `CaptureScene`
  (`SceneCaptureComponent2D.CaptureScene` (`self.SceneCaptureComponent2D`)))

(fn `CreateAutomapTexture`
  (returns (AutomapTexture :type "Texture2D Object Reference"))
  (`self.CaptureScene`)
  (bind _returnvalue (`GameplayUtilities.CreateAutomapTextureAsset` (`SceneCaptureComponent2D.TextureTarget` (`self.SceneCaptureComponent2D`)) (`self.AutomapName`)))
  (bind _output_get (set `self.AutomapTexture` _returnvalue))
  (return _output_get))

(fn `CreateTextureTarget`
  (bind (_boxextent_x _boxextent_y _boxextent_z) (`KismetMathLibrary.BreakVector` (`BoxComponent.BoxExtent` (`self.Bounds`))))
  (bind _returnvalue (`KismetMathLibrary.FFloor` (`KismetMathLibrary.MultiplyMultiply_FloatFloat` 2.0 (`KismetMathLibrary.Conv_IntToDouble` (`KismetMathLibrary.FCeil` (/ (`KismetMathLibrary.Loge` (/ (`KismetMathLibrary.FMax` _boxextent_x _boxextent_y _boxextent_z) (`self.UnitsPerPixel`))) (`KismetMathLibrary.Loge` 2.0)))))))
  (bind _returnvalue_2 (`CanvasRenderTarget2D.CreateCanvasRenderTarget2D` "/Script/Engine.CanvasRenderTarget2D" _returnvalue _returnvalue))
  (bind _output_get (set `SceneCaptureComponent2D.TextureTarget` _returnvalue_2 (`self.SceneCaptureComponent2D`)))
  (set `Texture.Filter` "TF_Nearest" _output_get)
  (`self.SetSceneCaptureToBounds`)
  (`KismetSystemLibrary.CollectGarbage`))

(fn `SetSceneCaptureToBounds`
  (bind (_boxextent_x _boxextent_y _boxextent_z) (`KismetMathLibrary.BreakVector` (`BoxComponent.BoxExtent` (`self.Bounds`))))
  (`SceneComponent.K2_SetRelativeLocationAndRotation` (`self.SceneCaptureComponent2D`) (`KismetMathLibrary.MakeVector` 0.0 0.0 _boxextent_z) (struct :`Pitch` -90.0) false false))

(fn `UserConstructionScript`)