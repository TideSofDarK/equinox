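; BP_Camera_Survival is a survival-mode camera that takes over player 0's view when a survival character sets off one of its triggers.
; On BeginPlay it binds to the CameraTriggerED event of every object in its Trigger array.
; When one fires with a BP_Character_Survival actor, the player controller cubic-blends its view target to this camera over BlendTime, with the outgoing view locked.
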(event `self.ReceiveBeginPlay`
  (for _array_element (`self.Trigger`)
    (add `/Game/FD10/Core/Survival/BP_CameraTrigger_Survival.CameraTriggerED` _array_element (delegate `OnOverlap`))))

(event `OnOverlap`
  (params (Actor :type "Actor Object Reference"))
  (if (`KismetMathLibrary.ClassIsChildOf` (`GameplayStatics.GetObjectClass` Actor) "/Game/FD10/Core/Survival/Character/BP_Character_Survival.BP_Character_Survival_C")
    (`PlayerController.SetViewTargetWithBlend` (`GameplayStatics.GetPlayerController` 0) self (`self.BlendTime`) "VTBlend_Cubic" 0.2 true)))

(fn `UserConstructionScript`)