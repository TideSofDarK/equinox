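; Survival player controller that owns slot-keyed inventory and stash item grids and opens their UI, plus pickup and examination widgets.
; An input-mode state (Ingame/UI/Cutscene) toggles pawn input, and item pickup also pauses the game until its widget closes.
; Saving converts the grids to actor maps and loading refills them through a cast macro.
; F-keys trigger debug save, load, item spawning and garbage collection; free-slot search functions are unfinished stubs.
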(event `Key|F10` :paused true
  (params (Key :type "Key Structure")))

(event `Key|F12` :paused true
  (params (Key :type "Key Structure"))
  (:`Pressed`
    (`KismetSystemLibrary.CollectGarbage`)))

(event `Key|F10`
  (params (Key :type "Key Structure"))
  (:`Pressed`
    (bind (_inventorygrid _stashgrid) (`self.SaveInventory`))
    (`FDSaveGame.SaveGame` _inventorygrid _stashgrid 1)))

(event `Key|F9`
  (params (Key :type "Key Structure"))
  (:`Pressed`
    (bind (_inventorygrid _stashgrid) (`FDSaveGame.LoadGame` 1))
    (`self.LoadInventory_Event` _inventorygrid _stashgrid)))

(event `LoadInventory_Event`
  (params (InventoryGrid :type "Map of IntVector Structure to SurvivalItemBase Object Reference") (StashGrid :type "Map of IntVector Structure to SurvivalItemBase Object Reference"))
  (`self.FillItemGrid` InventoryGrid (`self.InventoryGrid`)
    (:`Completed`
      (`self.FillItemGrid` StashGrid (`self.StashGrid`)))))

(event `Key|F8`
  (params (Key :type "Key Structure"))
  (:`Pressed`
    (bind _returnvalue (`self.SpawnPickedItem` "/Game/FD10/Items/Weapons/Sigismund/BP_Sigismund.BP_Sigismund_C"))
    (`self.AddItemToInventory` _returnvalue (make `IntVector` 0))
    (bind _returnvalue_2 (`self.SpawnPickedItem` "/Game/FD10/Items/Weapons/Sigismund/BP_Sigismund_Ammo.BP_Sigismund_Ammo_C"))
    (`self.AddItemToInventory` _returnvalue_2 (make `IntVector` 1))
    (set `/Game/FD10/Core/Survival/Items/BP_SurvivalItem.StackCount` 15 _returnvalue_2)
    (bind _returnvalue_3 (`self.SpawnPickedItem` "/Game/FD10/Items/Weapons/Shotgun/BP_Shotgun.BP_Shotgun_C"))
    (`self.AddItemToInventory` _returnvalue_3 (make `IntVector` 0 1))
    (bind _returnvalue_4 (`self.SpawnPickedItem` "/Game/FD10/Items/Pills/BP_PillsA.BP_PillsA_C"))
    (`self.AddItemToStash` _returnvalue_4 (make `IntVector` 0 1))))

(event `InputAction|Inventory`
  (params (Key :type "Key Structure"))
  (:`Pressed`
    (`self.SwitchOnInputMode`
      (:`Ingame`
        (`/Game/FD10/Core/Survival/HUD_Survival.OpenInventory_Event` (`/Game/FD10/Core/Survival/BPFL_SurvivalUtilities.GetSurvivalHud`) null)
        (`self.SetSurvivalInputMode_Event` "NewEnumerator1")))))

(event `self.ReceiveBeginPlay`
  (`WidgetBlueprintLibrary.SetInputMode_GameAndUIEx` self null))

(event `OnItemPickup_Event`
  (params (Item :type "/Game/FD10/Core/Survival/Items/BP_SurvivalItem Object Reference"))
  (`GameplayStatics.SetGamePaused` true)
  (`self.SetSurvivalInputMode_Event` "NewEnumerator1")
  (bind _returnvalue (`|CreateWidget` "/Game/FD10/Widgets/ItemPickup/WBP_ItemPickup.WBP_ItemPickup_C" self Item))
  (`UserWidget.AddToPlayerScreen` _returnvalue 0)
  (add `/Game/FD10/Widgets/ItemPickup/WBP_ItemPickup.ItemPickupED` _returnvalue (delegate `OnItemPickupClosed_Event`)))

(event `OnItemPickupClosed_Event`
  (`GameplayStatics.SetGamePaused` false)
  (`self.SetSurvivalInputMode_Event` "NewEnumerator0"))

(event `SetSurvivalInputMode_Event`
  (params (NewInputMode :type "/Game/FD10/Core/Survival/ESurvivalInputMode Enum" :default "NewEnumerator0"))
  (bind _output_get (set `self.InputMode` NewInputMode))
  (switch `/Game/FD10/Core/Survival/ESurvivalInputMode` _output_get
    (:`NewEnumerator0`
      (`self.EnableInput` (`/Game/FD10/Core/Survival/BPFL_SurvivalUtilities.GetSurvivalPlayerPawn`) self))
    (:`NewEnumerator1`
      (`self.DisableInput` (`/Game/FD10/Core/Survival/BPFL_SurvivalUtilities.GetSurvivalPlayerPawn`) self :!label _label))
    (:`NewEnumerator2`
      (goto _label))))

(event `self.ReceiveTick`
  (params (DeltaSeconds :type "Float (single-precision)")))

(fn `AddItemToInventory`
  (params (Item :type "/Game/FD10/Core/Survival/Items/BP_SurvivalItem Object Reference") (Slot :type "IntVector Structure"))
  (`BlueprintMapLibrary.Map_Add` (`self.InventoryGrid`) Slot Item))

(fn `AddItemToStash`
  (params (Item :type "/Game/FD10/Core/Survival/Items/BP_SurvivalItem Object Reference") (Slot :type "IntVector Structure"))
  (`BlueprintMapLibrary.Map_Add` (`self.StashGrid`) Slot Item))

(fn `ConvertItemGridToActorGrid`
  (params (ItemGrid :type "Map of IntVector Structure to /Game/FD10/Core/Survival/Items/BP_SurvivalItem Object Reference"))
  (returns (ActorGrid :type "Map of IntVector Structure to Actor Object Reference"))
  (locals (LocalActorGrid :type "Map of IntVector Structure to Actor Object Reference"))
  (bind _keys (`BlueprintMapLibrary.Map_Keys` ItemGrid))
  (for _array_element _keys
    (bind (_value _returnvalue) (`BlueprintMapLibrary.Map_Find` (`local.ItemGrid`) _array_element))
    (if _returnvalue
      (`BlueprintMapLibrary.Map_Add` (`local.LocalActorGrid`) _array_element _value)))
  (return (`local.LocalActorGrid`)))

(fn `FindFreeInventorySlot`
  (params (ItemClass :type "/Game/FD10/Core/Survival/Items/BP_SurvivalItem Class Reference"))
  (returns (bFound :type Boolean) (Slot :type "IntVector Structure"))
  (bind (_inventorysize_x _inventorysize_y) (break `IntVector` (`self.InventorySize`)))
  (for _ (range _inventorysize_y)
    (for _ (range _inventorysize_x)
      _)))

(fn `IsInventoryQuadFree`
  (params (Size :type "IntVector Structure") (Slot :type "IntVector Structure")))

(fn `OpenItemExaminationWithCloseCallback`
  (params (Item :type "/Game/FD10/Core/Survival/Items/BP_SurvivalItem Object Reference") (Event :type "Delegate (by ref)"))
  (bind _returnvalue (`|CreateWidget` "/Game/FD10/Widgets/Inventory/WBP_ItemExamination.WBP_ItemExamination_C" self Item))
  (`UserWidget.AddToPlayerScreen` _returnvalue 0)
  (add `/Game/FD10/Widgets/Inventory/WBP_ItemExamination.CloseED` _returnvalue Event)
  (`Widget.SetUserFocus` _returnvalue self)
  (return))

(fn `OpenStashWithCloseCallback`
  (params (Event :type "Delegate (by ref)"))
  (bind _returnvalue (`|CreateWidget` "/Game/FD10/Widgets/Inventory/WBP_Stash.WBP_Stash_C" self null))
  (`UserWidget.AddToPlayerScreen` _returnvalue 0)
  (add `/Game/FD10/Widgets/Inventory/WBP_Stash.StashED` _returnvalue Event)
  (return))

(fn `SaveInventory`
  (returns (InventoryGrid :type "Map of IntVector Structure to Actor Object Reference") (StashGrid :type "Map of IntVector Structure to Actor Object Reference"))
  (bind _actorgrid (`self.ConvertItemGridToActorGrid` (`self.InventoryGrid`)))
  (bind _actorgrid_2 (`self.ConvertItemGridToActorGrid` (`self.StashGrid`)))
  (return _actorgrid _actorgrid_2))

(fn `SpawnPickedItem`
  (params (ItemClass :type "/Game/FD10/Core/Survival/Items/BP_SurvivalItem Class Reference"))
  (returns (ReturnValue :type "/Game/FD10/Core/Survival/Items/BP_SurvivalItem Object Reference"))
  (bind _returnvalue (`GameplayStatics.GetPlayerPawn` 0))
  (bind _returnvalue_2 (`|SpawnActorFromClass` ItemClass (`KismetMathLibrary.MakeTransform` (0.0 0.0 0.0)) "AlwaysSpawn" "OverrideRootScale" null 1 null))
  (`/Engine/EditorBlueprintResources/StandardMacros.IsValid` _returnvalue
    (:`Is Valid`
      (`self.SetOwner` _returnvalue_2 _returnvalue))
    (:`Is Not Valid`
      _))
  (`SurvivalItemBase.OnPicked` _returnvalue_2)
  (return _returnvalue_2))

(fn `UserConstructionScript`)