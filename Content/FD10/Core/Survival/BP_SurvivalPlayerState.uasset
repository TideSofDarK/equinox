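; Survival player state that handles level startup, screen transitions, background music and save/load.
; On BeginPlay, if a level manifest exists, it transitions in, switches input modes, fades in music, initializes the HUD and loads slot 0.
; Pause-tolerant timelines drive music fades and the transition-out, with transitions using a post-process material and parameter collection centered on projected world positions.
; Saves store inventory, stash, actors to destroy and a scene-capture screenshot.
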(event `OnTransitionInFinished`
  (remove `self.OnTransitionFinished` (delegate `OnTransitionInFinished`))
  (`self.RemovePostProcessMaterial` "/Game/FD10/MaterialLibrary/M_Transition.M_Transition")
  (`/Game/FD10/Core/Survival/BP_SurvivalPlayerController.SetSurvivalInputMode` (`/Game/FD10/Core/Survival/BPFL_SurvivalUtilities.GetSurvivalPlayerController`) "NewEnumerator0"))

(event `self.ReceiveBeginPlay`
  (bind _returnvalue (`GameplayStatics.GetActorOfClass` "/Game/FD10/Core/Survival/Levels/BP_LevelManifest.BP_LevelManifest_C"))
  (bind _output_get (set `self.LevelManifest` _returnvalue))
  (`/Engine/EditorBlueprintResources/StandardMacros.IsValid` _output_get
    (:`Is Valid`
      (`|ExecutionSequence`
        (:`then_0`
          (`self.TransitionIn` (`self.GetPlayerPawnWorldLocationCentered`))
          (add `self.OnTransitionFinished` (delegate `OnTransitionInFinished`)))
        (:`then_1`
          (`/Game/FD10/Core/Survival/BP_SurvivalPlayerController.SetSurvivalInputMode` (`/Game/FD10/Core/Survival/BPFL_SurvivalUtilities.GetSurvivalPlayerController`) "NewEnumerator2"))
        (:`then_2`
          (`TimelineComponent.PlayFromStart` (`self.BGMFade`)))
        (:`then_3`
          (`/Game/FD10/Core/Survival/HUD_Survival.InitGeneralHUD` (`/Game/FD10/Core/Survival/BPFL_SurvivalUtilities.GetSurvivalHud`)))
        (:`then_4`
          (`self.LoadGameFromSlot` 0))))
    (:`Is Not Valid`
      (bind _returnvalue_2 (`GameplayStatics.GetCurrentLevelName` true))
      (`KismetSystemLibrary.PrintString` (`KismetStringLibrary.Concat_StrStr` "Level Manifest not found on level " _returnvalue_2) true true (struct :`R` 1.0 :`A` 1.0)))))

(fn `CaptureSaveGameScreenshot`
  (bind _returnvalue (`Controller.GetViewTarget` (`/Game/FD10/Core/Survival/BPFL_SurvivalUtilities.GetSurvivalPlayerController`)))
  (bind _returnvalue_2 (`AddComponent|NODE_AddSceneCaptureComponent2D-0`))
  (bind _output_get (set `self.ScreenshotCapture` _returnvalue_2))
  (`SceneCaptureComponent.HideActorComponents` _output_get (`GameplayStatics.GetPlayerPawn` 0) false)
  (set `SceneCaptureComponent.CaptureSource` "SCS_FinalColorHDR" _output_get)
  (set `SceneCaptureComponent.bCaptureEveryFrame` false (`self.ScreenshotCapture`))
  (set `SceneCaptureComponent.bCaptureOnMovement` false (`self.ScreenshotCapture`))
  (set `SceneCaptureComponent2D.FOVAngle` 60.0 (`self.ScreenshotCapture`))
  (`KismetArrayLibrary.Array_Add` (`SceneCaptureComponent.ShowFlagSettings` (`self.ScreenshotCapture`)) (make `EngineShowFlagsSetting` "BSP"))
  (`SceneComponent.K2_SetWorldLocationAndRotation` (`self.ScreenshotCapture`) (`self.K2_GetActorLocation` _returnvalue) (`self.K2_GetActorRotation` _returnvalue) false false)
  (bind _returnvalue_3 (`KismetRenderingLibrary.CreateRenderTarget2D` 256 256 "RTF_RGBA8" (struct :`A` 1.0) true))
  (set `SceneCaptureComponent2D.TextureTarget` _returnvalue_3 (`self.ScreenshotCapture`))
  (`SceneCaptureComponent2D.CaptureScene` (`self.ScreenshotCapture`)))

(fn `DestroyActorOnLoad`
  (params (ActorName :type String))
  (`KismetArrayLibrary.Array_AddUnique` (`self.ActorsToDestroy`) ActorName))

(fn `GetPlayerPawnWorldLocationCentered`
  (returns (Location :type "Vector Structure"))
  (return (+ (`self.K2_GetActorLocation` (`/Game/FD10/Core/Survival/BPFL_SurvivalUtilities.GetSurvivalPlayerPawn`)) (0.0 0.0 50.0))))

(fn `LoadGameFromSlot`
  (params (Slot :type Integer))
  (bind (_inventorygrid _stashgrid _equippeditem) (`FDSaveGame.LoadGame` self Slot))
  (`/Game/FD10/Core/Survival/BP_SurvivalPlayerController.LoadInventoryAndStash` (`/Game/FD10/Core/Survival/BPFL_SurvivalUtilities.GetSurvivalPlayerController`) _inventorygrid _stashgrid)
  (bind _asbp_weapon (cast `/Game/FD10/Core/Survival/Items/BP_Weapon` _equippeditem)
    (:`then`
      (`/Game/FD10/Core/Survival/Characters/BP_SurvivalMainCharacter.EquipWeapon` (`/Game/FD10/Core/Survival/BPFL_SurvivalUtilities.GetSurvivalPlayerPawn`) _asbp_weapon))
    (:`CastFailed`
      _))
  (`KismetSystemLibrary.CollectGarbage`))

(fn `SaveGameToSlot`
  (params (Slot :type Integer))
  (bind (_inventorygrid _stashgrid) (`/Game/FD10/Core/Survival/BP_SurvivalPlayerController.ConvertInventoryAndStashToActorGrids` (`/Game/FD10/Core/Survival/BPFL_SurvivalUtilities.GetSurvivalPlayerController`)))
  (`FDSaveGame.SaveGame` self _inventorygrid _stashgrid (`self.ActorsToDestroy`) (`local.Slot`) (`self.ScreenshotCapture`))
  (return))

(fn `SetBGMAndPlay`
  (params (NewBGM :type "SoundBase Object Reference"))
  (`AudioComponent.SetSound` (`self.BGM`) NewBGM)
  (`AudioComponent.Play` (`self.BGM`) 0.0))

(fn `SetBGMPaused`
  (params (bIsPaused :type Boolean) (FadeTime :type "Float (double-precision)"))
  (`AudioComponent.SetPaused` (`self.BGM`) bIsPaused)
  (if (> (`local.FadeTime`) 0.0)
    (`TimelineComponent.SetPlayRate` (`self.BGMFade`) (`local.FadeTime`))
    (if (`local.bIsPaused`)
      (`TimelineComponent.ReverseFromEnd` (`self.BGMFade`))
      (else
        (`TimelineComponent.PlayFromStart` (`self.BGMFade`))))))

(fn `TransitionIn`
  (params (WorldPosition :type "Vector Structure (by ref)"))
  (bind (_returnvalue_x _returnvalue_y) (`self.WorldToViewport` WorldPosition))
  (`|ExecutionSequence`
    (:`then_0`
      (`TimelineComponent.ReverseFromEnd` (`self.TransitionInTimeline`)))
    (:`then_1`
      (`KismetMaterialLibrary.SetVectorParameterValue` "/Game/FD10/MaterialLibrary/MPC_Transition.MPC_Transition" "RadialBlurCenter" (make `LinearColor` _returnvalue_x _returnvalue_y)))
    (:`then_2`
      (`self.AddPostProcessMaterial` "/Game/FD10/MaterialLibrary/M_Transition.M_Transition"))))

(fn `TransitionOut`
  (params (WorldPosition :type "Vector Structure (by ref)"))
  (bind (_returnvalue_x _returnvalue_y) (`self.WorldToViewport` WorldPosition))
  (`GameplayStatics.PlaySound2D` "/Game/FD10/Audio/A_Transition.A_Transition" 1.0 (`KismetMathLibrary.RandomFloatInRange` 0.85 1.05) 0.0 null null)
  (`KismetMaterialLibrary.SetVectorParameterValue` "/Game/FD10/MaterialLibrary/MPC_Transition.MPC_Transition" "RadialBlurCenter" (make `LinearColor` _returnvalue_x _returnvalue_y))
  (`TimelineComponent.SetPlayRate` (`self.TransitionOutTimeline`) 1.0)
  (`TimelineComponent.PlayFromStart` (`self.TransitionOutTimeline`))
  (`self.AddPostProcessMaterial` "/Game/FD10/MaterialLibrary/M_Transition.M_Transition"))

(fn `UserConstructionScript`
  (`ActorComponent.SetTickableWhenPaused` (`self.BGMFade`) true)
  (`ActorComponent.SetTickableWhenPaused` (`self.TransitionOutTimeline`) true))