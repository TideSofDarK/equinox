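; BP_SurvivalCamera is a camera actor for survival gameplay that takes over the player's view when one of its triggers is overlapped.
; On BeginPlay it binds every trigger and, if flagged as the initial camera, activates for the player pawn.
; An overlap disables the previous survival camera's tick, then activation caches the character, cubic-blends the view target and enables this camera's tick.
; Re-activation while already active is optional.
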(event `self.ReceiveBeginPlay`
  (if (`self.bInitialCamera`)
    (`self.OnActivate_Event` (`/Game/FD10/Core/Survival/BPFL_SurvivalUtilities.GetSurvivalPlayerPawn`)))
  (for _array_element (`self.Trigger`)
    (add `/Game/FD10/Core/Survival/Camera/BP_SurvivalCameraTrigger.OnCameraTriggerOverlap` _array_element (delegate `OnOverlap_Event`))))

(event `OnOverlap_Event`
  (params (Character :type "/Game/FD10/Core/Survival/Characters/BP_SurvivalCharacterBase Object Reference"))
  (if (or (!= (`Controller.GetViewTarget` (`/Game/FD10/Core/Survival/BPFL_SurvivalUtilities.GetSurvivalPlayerController`)) self) (`self.bActivateEvenIfActive`))
    (bind _asbp_survival_camera (cast `/Game/FD10/Core/Survival/Camera/BP_SurvivalCamera` (`Controller.GetViewTarget` (`/Game/FD10/Core/Survival/BPFL_SurvivalUtilities.GetSurvivalPlayerController`)))
      (:`then`
        (`self.SetActorTickEnabled` _asbp_survival_camera false))
      (:`CastFailed`
        _))
    (`self.OnActivate_Event` Character)))

(event `OnActivate_Event`
  (params (Character :type "/Game/FD10/Core/Survival/Characters/BP_SurvivalCharacterBase Object Reference"))
  (set `self.CachedCharacter` Character)
  (`PlayerController.SetViewTargetWithBlend` (`GameplayStatics.GetPlayerController` 0) self (`self.BlendTime`) "VTBlend_Cubic" 0.2 true)
  (`self.SetActorTickEnabled` true))

(fn `UserConstructionScript`)