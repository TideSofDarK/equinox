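; BP_SurvivalCameraTrigger is a survival-mode camera trigger volume that broadcasts OnCameraTriggerOverlap while a BP_SurvivalMainCharacter is inside it.
; Begin overlap stores the character and enables Tick, while any end overlap clears the reference and disables Tick.
; Each Tick fires the dispatcher with that character, filtered by TriggerType: always, or only when the character is at/above or below the trigger's origin height.
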(event `self.ReceiveTick`
  (params (DeltaSeconds :type "Float (single-precision)"))
  (bind (_returnvalue_x _returnvalue_y _returnvalue_z) (`KismetMathLibrary.BreakVector` (`self.K2_GetActorLocation`)))
  (bind (_returnvalue_x_2 _returnvalue_y_2 _returnvalue_z_2) (`KismetMathLibrary.BreakVector` (`self.K2_GetActorLocation` (`self.OverlappingCharacter`))))
  (bind _returnvalue (>= _returnvalue_z_2 _returnvalue_z))
  (switch `/Game/FD10/Core/Survival/Camera/ECameraTriggerRestriction` (`self.TriggerType`)
    (:`NewEnumerator0`
      (`self.OnCameraTriggerOverlap` (`self.OverlappingCharacter`) :!label _label))
    (:`NewEnumerator1`
      (if _returnvalue
        (goto _label)))
    (:`NewEnumerator2`
      (if (not _returnvalue)
        (goto _label)))))

(event `self.ReceiveActorBeginOverlap`
  (params (OtherActor :type "Actor Object Reference"))
  (bind _asbp_survival_main_character (cast `/Game/FD10/Core/Survival/Characters/BP_SurvivalMainCharacter` OtherActor))
  (set `self.OverlappingCharacter` _asbp_survival_main_character)
  (`self.SetActorTickEnabled` true))

(event `self.ReceiveActorEndOverlap`
  (params (OtherActor :type "Actor Object Reference"))
  (set `self.OverlappingCharacter` null)
  (`self.SetActorTickEnabled` false))

(fn `UserConstructionScript`)