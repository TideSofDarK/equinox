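; Survival-mode camera that rides a spline to follow the cached character, snapping into place on activation and easing every tick.
; Position is the spline point nearest a spot offset from the character toward the camera, so the camera trails at a distance.
; Rotation blends the spline direction, flipped to match the camera's current facing, with a look-at slightly above the character, weighted toward the look-at.
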(event `self.ReceiveBeginPlay`
  (`parent.ReceiveBeginPlay`))

(event `self.ReceiveTick`
  (params (DeltaSeconds :type "Float (single-precision)"))
  (`parent.ReceiveTick` DeltaSeconds)
  (`self.OnUpdateCamera_Event` (* DeltaSeconds (`self.RotationEaseRate`)) (* DeltaSeconds (`self.LocationEaseRate`))))

(event `self.OnActivate_Event`
  (params (Character :type "/Game/FD10/Core/Survival/Characters/BP_SurvivalCharacterBase Object Reference"))
  (`parent.OnActivate_Event` Character)
  (`self.OnUpdateCamera_Event` 1.0 1.0 true))

(event `OnUpdateCamera_Event`
  (params (RotationEaseAlpha :type "Float (double-precision)") (LocationEaseAlpha :type "Float (double-precision)") (bIsImmediate :type Boolean))
  (bind _returnvalue (`SplineComponent.FindDirectionClosestToWorldLocation` (`self.Spline`) (`self.K2_GetActorLocation` (`self.CachedCharacter`)) "World"))
  (bind _returnvalue_2 (`KismetMathLibrary.RLerp` (`KismetMathLibrary.MakeRotFromX` (select `bool` (< (`KismetMathLibrary.Dot_VectorVector` _returnvalue (`SceneComponent.GetForwardVector` (`self.Camera`))) 0.0) :`false` _returnvalue :`true` (* _returnvalue -1.0))) (`KismetMathLibrary.FindLookAtRotation` (`SceneComponent.K2_GetComponentLocation` (`self.Camera`)) (+ (`self.K2_GetActorLocation` (`self.CachedCharacter`)) (0.0 0.0 50.0))) 0.75 true))
  (bind _cachedcharacter (`self.CachedCharacter`)
    (:`then`
      (bind _returnvalue_3 (`SplineComponent.FindLocationClosestToWorldLocation` (`self.Spline`) (+ (`self.K2_GetActorLocation` _cachedcharacter) (* (`KismetMathLibrary.Normal` (- (`SceneComponent.K2_GetComponentLocation` (`self.Camera`)) (`self.K2_GetActorLocation` (`self.CachedCharacter`)))) 300.0)) "World"))
      (`SceneComponent.K2_SetWorldLocationAndRotation` (`self.Camera`) (select `bool` bIsImmediate :`false` (`|EaseFunction` "EaseInOut" LocationEaseAlpha (`SceneComponent.K2_GetComponentLocation` (`self.Camera`)) _returnvalue_3 1.5) :`true` _returnvalue_3) (select `bool` bIsImmediate :`false` (`|EaseFunction` "CircularIn" RotationEaseAlpha (`SceneComponent.K2_GetComponentRotation` (`self.Camera`)) _returnvalue_2) :`true` _returnvalue_2) false false))
    (:`else`)))

(fn `UserConstructionScript`
  (`parent.UserConstructionScript`))