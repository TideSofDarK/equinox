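; Survival camera variant that dollies its camera along the actor's forward direction based on the cached character's distance from the camera actor.
; Distance over CharacterRange, clamped to 0–1, blends from the actor's location to a point ZoomRange ahead, with an XY mode that keeps the actor's height.
; Activation snaps the camera there; Tick eases toward it using ZoomingEaseRate scaled by delta time.
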(event `self.OnActivate_Event`
  (params (Character :type "/Game/FD10/Core/Survival/Characters/BP_SurvivalCharacterBase Object Reference"))
  (`parent.OnActivate_Event` Character)
  (`self.UpdateCameraZoom` 0.0 true))

(event `self.ReceiveTick`
  (params (DeltaSeconds :type "Float (single-precision)"))
  (`parent.ReceiveTick` DeltaSeconds)
  (`self.UpdateCameraZoom` (* DeltaSeconds (`self.ZoomingEaseRate`))))

(fn `UpdateCameraZoom`
  (params (ZoomingEaseAlpha :type "Float (double-precision)") (bIsImmediate :type Boolean))
  (bind _returnvalue (`self.K2_GetActorLocation`))
  (bind _returnvalue_2 (+ (* (`self.GetActorForwardVector`) (`self.ZoomRange`)) _returnvalue))
  (bind _returnvalue_3 (`KismetMathLibrary.VLerp` (`self.K2_GetActorLocation`) (select `/Game/FD10/Core/Survival/Camera/ECameraZoomMode` (`self.CameraZoomMode`) :`NewEnumerator0` _returnvalue_2 :`NewEnumerator1` (`KismetMathLibrary.MakeVector` (.x _returnvalue_2) (.y _returnvalue_2) (.z _returnvalue))) (`KismetMathLibrary.FClamp` (/ (`KismetMathLibrary.Vector_Distance` (`self.K2_GetActorLocation` (`self.CachedCharacter`)) (`self.K2_GetActorLocation`)) (`self.CharacterRange`)))))
  (`self.CachedCharacter`
    (:`then`
      (`SceneComponent.K2_SetWorldLocation` (`self.Camera`) (select `bool` bIsImmediate :`false` (`|EaseFunction` "Linear" ZoomingEaseAlpha (`SceneComponent.K2_GetComponentLocation` (`self.Camera`)) _returnvalue_3) :`true` _returnvalue_3) false false))
    (:`else`)))

(fn `UserConstructionScript`
  (`parent.UserConstructionScript`))