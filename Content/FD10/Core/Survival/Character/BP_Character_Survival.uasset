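; Player character for a survival game, with tank-style movement, weapon handling and interaction.
; Forward input moves along control yaw, or pitches the view while aiming; yaw drift from the body triggers turn-in-place montages, and a quick-turn montage drags control rotation along.
; Primary fires the equipped weapon when aiming, alternating dry-fire and inventory-based reload when firing fails, otherwise interacts via a forward capsule trace.
; Also handles walk/run gait, weapon attachment and timed look-at targets.
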(event `InputAxis|MoveForward/Backwards`
  (params (AxisValue :type "Float (single-precision)"))
  (bind (_returnvalue_roll _returnvalue_pitch _returnvalue_yaw) (`KismetMathLibrary.BreakRotator` (`self.GetControlRotation`)))
  (bind (_returnvalue_roll_2 _returnvalue_pitch_2 _returnvalue_yaw_2) (`KismetMathLibrary.BreakRotator` (`self.GetControlRotation`)))
  (if (`self.bAiming`)
    (`self.AddControllerPitchInput` (* AxisValue (`self.RotateRate`) (`GameplayStatics.GetWorldDeltaSeconds`) -1.0))
    (set `self.InputMove` 0.0)
    (else
      (bind _output_get (set `self.InputMove` AxisValue))
      (`self.AddMovementInput` (`KismetMathLibrary.Conv_RotatorToVector` (`KismetMathLibrary.MakeRotator` 0.0 0.0 _returnvalue_yaw)) (* _output_get (`self.MovementRate`) (`GameplayStatics.GetWorldDeltaSeconds`)))
      (if (> (`KismetMathLibrary.Abs` (`self.InputMove`)) 0.0)
        (`self.K2_SetActorRotation` (`KismetMathLibrary.RInterpTo_Constant` (`self.K2_GetActorRotation`) (`KismetMathLibrary.MakeRotator` 0.0 0.0 _returnvalue_yaw_2) (`GameplayStatics.GetWorldDeltaSeconds`) 150.0))))))

(event `InputAxis|MoveRight/Left`
  (params (AxisValue :type "Float (single-precision)"))
  (set `self.InputRotation` AxisValue)
  (`self.AddControllerYawInput` (* (`self.InputRotation`) (`self.RotateRate`) (`GameplayStatics.GetWorldDeltaSeconds`))))

(event `InputAction|WalkAction`
  (params (Key :type "Key Structure"))
  (:`Pressed`
    (set `self.Gait` "NewEnumerator1")
    (set `CharacterMovementComponent.MaxWalkSpeed` (`self.RunningSpeed`) (`self.CharacterMovement`)))
  (:`Released`
    (set `self.Gait` "NewEnumerator0")
    (set `CharacterMovementComponent.MaxWalkSpeed` (`self.WalkingSpeed`) (`self.CharacterMovement`) :!label _label)))

(event `SetInitialWalkingSpeed_Event`
  (goto _label))

(event `InputAction|TurnAround`
  (params (Key :type "Key Structure"))
  (:`Pressed`
    (if (not (`AnimInstance.IsAnyMontagePlaying` (`SkeletalMeshComponent.GetAnimInstance` (`self.Mesh`))))
      (`|PlayMontage` (`self.Mesh`) (select `bool` (`KismetMathLibrary.RandomBool`) :`false` "/Game/FD10/Characters/MocapOnline/Animations/TurnInPlace/A_TurnInPlace_L180_RM_Montage.A_TurnInPlace_L180_RM_Montage" :`true` "/Game/FD10/Characters/MocapOnline/Animations/TurnInPlace/A_TurnInPlace_R180_RM_Montage.A_TurnInPlace_R180_RM_Montage" :!type "AnimMontage Object Reference")
        (:`then`
          (set `self.bOrientControlsToMontage` true))
        (:`OnCompleted`
          (set `self.bOrientControlsToMontage` false))))))

(event `self.ReceiveBeginPlay`
  (`self.SetInitialWalkingSpeed_Event`))

(event `self.ReceiveTick`
  (params (DeltaSeconds :type "Float (single-precision)"))
  (bind (_returnvalue_roll _returnvalue_pitch _returnvalue_yaw) (`KismetMathLibrary.BreakRotator` (`self.GetControlRotation`)))
  (bind _rotateinplacethreshold (`self.RotateInPlaceThreshold`))
  (bind _returnvalue (`SkeletalMeshComponent.GetAnimInstance` (`self.Mesh`)))
  (bind _returnvalue_2 (`SkeletalMeshComponent.GetAnimInstance` (`self.Mesh`)))
  (bind (_returnvalue_roll_2 _returnvalue_pitch_2 _returnvalue_yaw_2) (`KismetMathLibrary.BreakRotator` (`KismetMathLibrary.NormalizedDeltaRotator` (`self.GetControlRotation`) (`self.K2_GetActorRotation`))))
  (`|ExecutionSequence`
    (:`then_0`
      (bind (_outhit_hitactor _returnvalue_3) (`self.HitForInteractableObjects`))
      (if _returnvalue_3
        (set `self.InteractTarget` (`self.GetComponentByClass` _outhit_hitactor "/Game/FD10/Core/Components/BP_InteractableComponent.BP_InteractableComponent_C"))
        (else
          (set `self.InteractTarget` null))))
    (:`then_1`
      (`SceneComponent.K2_SetWorldRotation` (`self.Arrow2`) (`self.GetControlRotation`) false false))
    (:`then_2`
      (if (`self.bOrientControlsToMontage`)
        (`Controller.SetControlRotation` (`self.GetController`) (`KismetMathLibrary.RInterpTo_Constant` (`self.K2_GetActorRotation`) (`KismetMathLibrary.MakeRotator` 0.0 0.0 _returnvalue_yaw) (`GameplayStatics.GetWorldDeltaSeconds`) 150.0))
        (else
          (`|ExecutionSequence`
            (:`then_0`
              (if (< _returnvalue_yaw_2 (* -1.0 _rotateinplacethreshold))
                (if (not (`AnimInstance.Montage_IsPlaying` _returnvalue "/Game/FD10/Characters/MocapOnline/Animations/TurnInPlace/A_TurnInPlace_L_Loop_RM_Montage.A_TurnInPlace_L_Loop_RM_Montage"))
                  (`|PlayMontage` (`self.Mesh`) "/Game/FD10/Characters/MocapOnline/Animations/TurnInPlace/A_TurnInPlace_L_Loop_RM_Montage.A_TurnInPlace_L_Loop_RM_Montage"))
                (else
                  (`AnimInstance.Montage_Stop` _returnvalue 0.3 "/Game/FD10/Characters/MocapOnline/Animations/TurnInPlace/A_TurnInPlace_L_Loop_RM_Montage.A_TurnInPlace_L_Loop_RM_Montage"))))
            (:`then_1`
              (if (> _returnvalue_yaw_2 _rotateinplacethreshold)
                (if (not (`AnimInstance.Montage_IsPlaying` _returnvalue_2 "/Game/FD10/Characters/MocapOnline/Animations/TurnInPlace/A_TurnInPlace_R_Loop_RM_Montage.A_TurnInPlace_R_Loop_RM_Montage"))
                  (`|PlayMontage` (`self.Mesh`) "/Game/FD10/Characters/MocapOnline/Animations/TurnInPlace/A_TurnInPlace_R_Loop_RM_Montage.A_TurnInPlace_R_Loop_RM_Montage"))
                (else
                  (`AnimInstance.Montage_Stop` _returnvalue_2 0.3 "/Game/FD10/Characters/MocapOnline/Animations/TurnInPlace/A_TurnInPlace_R_Loop_RM_Montage.A_TurnInPlace_R_Loop_RM_Montage"))))))))))

(event `InputAction|Secondary`
  (params (Key :type "Key Structure"))
  (bind (_returnvalue_roll _returnvalue_pitch _returnvalue_yaw) (`KismetMathLibrary.BreakRotator` (`self.GetControlRotation`)))
  (bind _equippedweapon (`self.EquippedWeapon`))
  (:`Pressed`
    (`/Engine/EditorBlueprintResources/StandardMacros.IsValid` _equippedweapon
      (:`Is Valid`
        (set `self.bAiming` true))))
  (:`Released`
    (`/Engine/EditorBlueprintResources/StandardMacros.IsValid` _equippedweapon
      (:`Is Valid`
        (set `self.bAiming` false)
        (`Controller.SetControlRotation` (`self.GetController`) (`KismetMathLibrary.MakeRotator` _returnvalue_roll 0.0 _returnvalue_yaw))))))

(event `InputAction|Primary`
  (params (Key :type "Key Structure"))
  (:`Pressed`
    (if (and (`self.bAiming`) (not (`AnimInstance.IsAnyMontagePlaying` (`SkeletalMeshComponent.GetAnimInstance` (`self.Mesh`)))))
      (`/Engine/EditorBlueprintResources/StandardMacros.IsValid` (`self.EquippedWeapon`)
        (:`Is Valid`
          (bind _bsuccess (`/Game/FD10/Core/Survival/Items/BP_Weapon.Fire` (`self.EquippedWeapon`)))
          (if _bsuccess
            (`|PlayMontage` (`self.Mesh`) "/Game/FD10/Characters/MocapOnline/Animations/Fire/A_Pistol_Fire_Montage.A_Pistol_Fire_Montage")
            (else
              (`/Engine/EditorBlueprintResources/StandardMacros.FlipFlop`
                (:`A`
                  (`/Game/FD10/Core/Survival/Items/BP_Weapon.PlayOutOfAmmoSound` (`self.EquippedWeapon`)))
                (:`B`
                  (bind _playercontrollersurvival (`/Game/FD10/Core/Survival/BPML_Shortcuts_Survival.GetSurvivalPlayerController`)
                    (:`Success`
                      (bind _batleastonebullet (`/Game/FD10/Core/Survival/Items/BP_Weapon.Reload` (`self.EquippedWeapon`) (`/Game/FD10/Core/BP_PlayerController_Survival.InventoryGrid` _playercontrollersurvival)))
                      (if _batleastonebullet
                        (`|PlayMontage` (`self.Mesh`) "/Game/FD10/Characters/MocapOnline/Animations/Fire/A_Pistol_Reload_Montage.A_Pistol_Reload_Montage"
                          (:`then`
                            (set `self.bReloading` true))
                          (:`OnCompleted`
                            (set `self.bReloading` false)))
                        (else
                          (`/Game/FD10/Core/Survival/Items/BP_Weapon.PlayOutOfAmmoSound` (`self.EquippedWeapon`))))))))))))
      (else
        (bind (_outhit_hitactor _returnvalue) (`self.HitForInteractableObjects`))
        (if _returnvalue
          (bind _returnvalue_2 (`self.GetComponentByClass` _outhit_hitactor "/Game/FD10/Core/Components/BP_InteractableComponent.BP_InteractableComponent_C"))
          (`/Engine/EditorBlueprintResources/StandardMacros.IsValid` _returnvalue_2
            (:`Is Valid`
              (`/Game/FD10/Core/Components/BP_InteractableComponent.OnInteract` _returnvalue_2))))))))

(event `LookAtTarget_Event`
  (params (LookAtLocation :type "Vector Structure") (Duration :type "Float (double-precision)"))
  (`KismetSystemLibrary.K2_ClearAndInvalidateTimerHandle` (`self.LookAtLocationTimer`))
  (set `self.LookAtLocation` LookAtLocation)
  (set `self.bLookingAtLocation` true)
  (bind _returnvalue (`KismetSystemLibrary.K2_SetTimerDelegate` (delegate `CancelLookAtLocation_Event`) Duration))
  (set `self.LookAtLocationTimer` _returnvalue))

(event `CancelLookAtLocation_Event`
  (set `self.bLookingAtLocation` false)
  (`KismetSystemLibrary.K2_ClearAndInvalidateTimerHandle` (`self.LookAtLocationTimer`)))

(fn `EquipWeapon`
  (params (Weapon :type "/Game/FD10/Core/Survival/Items/BP_Weapon Object Reference"))
  (`/Engine/EditorBlueprintResources/StandardMacros.IsValid` (`self.EquippedWeapon`)
    (:`Is Valid`
      (`self.UnequipWeapon`))
    (:`Is Not Valid`
      _))
  (bind _output_get (set `self.EquippedWeapon` Weapon))
  (`self.K2_AttachToComponent` _output_get (`self.Mesh`) (`/Game/FD10/Core/Survival/Items/BP_Weapon.AttachSocket` _output_get) "KeepRelative" "KeepRelative" "KeepRelative" true)
  (`self.SetActorHiddenInGame` _output_get false))

(fn `UnequipWeapon`
  (`/Game/FD10/Core/Survival/Items/BP_Item_Survival.OnPostPickup_Event` (`self.EquippedWeapon`))
  (set `self.EquippedWeapon` null))

(fn `UserConstructionScript`)