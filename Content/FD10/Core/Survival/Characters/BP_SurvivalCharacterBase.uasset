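; Base character for the Survival mode, providing physical hit reactions, a visibility toggle and a brief tick-while-paused helper.
; Hits on non-root bones, when enabled, simulate physics below that bone and apply an impulse while a timeline drives the blend weight.
; When the timeline ends, physics is switched off unless the character is dead.
; The pause helper makes actor and mesh tickable for about one frame using a short retriggerable delay.
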(event `self.ReceiveBeginPlay`
  (set `self.DefaultAnimInstance` (`SkeletalMeshComponent.GetAnimInstance` (`self.Mesh`))))

(event `/Game/FD10/Core/Survival/Characters/BPI_HitReaction.HitReaction`
  (params (Bone :type Name) (Direction :type "Vector Structure"))
  (if (`self.bEnableHitReaction`)
    (if (!= Bone (`self.RootBoneName`))
      (if (`self.bIsReactingToHit`)
        _
        (else
          _))
      (set `self.bIsReactingToHit` true)
      (set `self.HitReactionBone` Bone)
      (`|ExecutionSequence`
        (:`then_0`
          (`SkeletalMeshComponent.SetAllBodiesBelowSimulatePhysics` (`self.Mesh`) (`self.HitReactionBone`) true true)
          (bind (_direction _alpha) (`Timeline|HitReactionTimeline` :!via `PlayFromStart`)
            (:`Update`
              (set `self.HitReactionBlendAlpha` _alpha)
              (`SkeletalMeshComponent.SetAllBodiesBelowPhysicsBlendWeight` (`self.Mesh`) (`self.HitReactionBone`) (`self.HitReactionBlendAlpha`) false true))
            (:`Finished`
              (if (not (`self.bIsDead`))
                (`SkeletalMeshComponent.SetAllBodiesPhysicsBlendWeight` (`self.Mesh`) 0.0 false)
                (`SkeletalMeshComponent.SetAllBodiesSimulatePhysics` (`self.Mesh`) false))
              (set `self.bIsReactingToHit` false))))
        (:`then_1`
          (`PrimitiveComponent.AddImpulse` (`self.Mesh`) (* Direction 1200.0) (`self.HitReactionBone`) true))))))

(event `TickForOneFrameDuringPause_Event`
  (`ActorComponent.SetTickableWhenPaused` (`self.Mesh`) true)
  (`self.SetTickableWhenPaused` true)
  (`KismetSystemLibrary.RetriggerableDelay` 0.03)
  (`self.SetTickableWhenPaused` false)
  (`ActorComponent.SetTickableWhenPaused` (`self.Mesh`) false))

(fn `SetCharacterVisibility`
  (params (bNewVisibility :type Boolean))
  (`SceneComponent.SetVisibility` (`self.CapsuleComponent`) bNewVisibility true))

(fn `UserConstructionScript`)