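; Player character for a survival game, with tank-style movement, walk/run gaits and montage-driven 180-degree turns.
; Tick capsule-traces for an interactable component to set InteractTarget.
; Primary interacts, or while aiming fires the attached weapon, alternating dry-fire sound and inventory-grid reload when firing fails.
; Also handles weapon equip/unequip and a timed look-at location; the legacy turn-in-place logic never runs.
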(event `InputAxis|MoveForward/Backwards`
  (params (AxisValue :type "Float (single-precision)"))
  (bind (_returnvalue_roll _returnvalue_pitch _returnvalue_yaw) (`KismetMathLibrary.BreakRotator` (`self.GetControlRotation`)))
  (if (`self.bTurningInPlace`)
    _
    (elif (not (`self.bAiming`))
      (bind _output_get (set `self.InputMove` AxisValue))
      (if (< _output_get 0.0)
        (set `CharacterMovementComponent.MaxWalkSpeed` (`self.WalkingSpeed`) (`self.CharacterMovement`))
        (else
          (`self.SetGait` (`self.Gait`))))
      (`self.AddMovementInput` (`KismetMathLibrary.Conv_RotatorToVector` (`KismetMathLibrary.MakeRotator` 0.0 0.0 _returnvalue_yaw)) (* _output_get (`self.MovementRate`) (`GameplayStatics.GetWorldDeltaSeconds`))))))

(event `InputAxis|MoveRight/Left`
  (params (AxisValue :type "Float (single-precision)"))
  (if (not (`self.bTurningInPlace`))
    (set `self.InputRotation` AxisValue)
    (`self.AddControllerYawInput` (* (`self.InputRotation`) (`self.RotateRate`) (`GameplayStatics.GetWorldDeltaSeconds`)))))

(event `InputAction|WalkAction`
  (params (Key :type "Key Structure"))
  (:`Pressed`
    (if (>= (`self.InputMove`) 0.0)
      (`self.SetGait` "NewEnumerator1")))
  (:`Released`
    (`self.SetGait` "NewEnumerator0" :!label _label)))

(event `SetInitialWalkingSpeed_Event`
  (goto _label))

(event `InputAction|TurnAround`
  (params (Key :type "Key Structure"))
  (:`Pressed`
    (if (not (`AnimInstance.IsAnyMontagePlaying` (`SkeletalMeshComponent.GetAnimInstance` (`self.Mesh`))))
      (set `self.bOrientControlsToMontage` true)
      (`|PlayMontage` (`self.Mesh`) (select `bool` (`KismetMathLibrary.RandomBool`) :`false` "/Game/FD10/Characters/July/Animations/TurnInPlace/A_RotateLeft180_Montage.A_RotateLeft180_Montage" :`true` "/Game/FD10/Characters/July/Animations/TurnInPlace/A_RotateRight180_Montage.A_RotateRight180_Montage" :!type "AnimMontage Object Reference")
        (:`then`
          (set `self.bTurningInPlace` true)
          (set `self.bUseControllerRotationYaw` false))
        (:`OnCompleted`
          (set `self.bTurningInPlace` false)
          (set `self.bUseControllerRotationYaw` true)
          (set `self.bOrientControlsToMontage` true))))))

(event `self.ReceiveBeginPlay`
  (`self.SetInitialWalkingSpeed_Event`))

(event `self.ReceiveTick`
  (params (DeltaSeconds :type "Float (single-precision)"))
  (if (`self.IsControlled`)
    (bind (_outhit_hitactor _returnvalue) (`self.HitForInteractableObjects`))
    (if _returnvalue
      (set `self.InteractTarget` (`self.GetComponentByClass` _outhit_hitactor "/Game/FD10/Core/Survival/Components/BP_InteractableComponent.BP_InteractableComponent_C"))
      (else
        (set `self.InteractTarget` null)))
    (else
      (set `self.InteractTarget` null))))

(event `InputAction|Secondary`
  (params (Key :type "Key Structure"))
  (bind (_returnvalue_roll _returnvalue_pitch _returnvalue_yaw) (`KismetMathLibrary.BreakRotator` (`self.GetControlRotation`)))
  (bind _equippedweapon (`self.EquippedWeapon`))
  (:`Pressed`
    (`/Engine/EditorBlueprintResources/StandardMacros.IsValid` _equippedweapon
      (:`Is Valid`
        (set `self.bAiming` true))))
  (:`Released`
    (`/Engine/EditorBlueprintResources/StandardMacros.IsValid` _equippedweapon
      (:`Is Valid`
        (set `self.bAiming` false)
        (`Controller.SetControlRotation` (`self.GetController`) (`KismetMathLibrary.MakeRotator` _returnvalue_roll 0.0 _returnvalue_yaw))))))

(event `InputAction|Primary`
  (params (Key :type "Key Structure"))
  (:`Pressed`
    (if (and (`self.bAiming`) (not (`AnimInstance.IsAnyMontagePlaying` (`SkeletalMeshComponent.GetAnimInstance` (`self.Mesh`)))))
      (`/Engine/EditorBlueprintResources/StandardMacros.IsValid` (`self.EquippedWeapon`)
        (:`Is Valid`
          (bind _bsuccess (`/Game/FD10/Core/Survival/Items/BP_Weapon.Fire` (`self.EquippedWeapon`)))
          (if _bsuccess
            (`|PlayMontage` (`self.Mesh`) "/Game/FD10/Characters/MocapOnline/Animations/Fire/A_Pistol_Fire_Montage.A_Pistol_Fire_Montage")
            (else
              (`/Engine/EditorBlueprintResources/StandardMacros.FlipFlop`
                (:`A`
                  (`/Game/FD10/Core/Survival/Items/BP_Weapon.PlayOutOfAmmoSound` (`self.EquippedWeapon`)))
                (:`B`
                  (bind _batleastonebullet (`/Game/FD10/Core/Survival/Items/BP_Weapon.Reload` (`self.EquippedWeapon`) (`/Game/FD10/Core/Survival/BP_SurvivalPlayerController.InventoryGrid` (`/Game/FD10/Core/Survival/BPFL_SurvivalUtilities.GetSurvivalPlayerController`))))
                  (if _batleastonebullet
                    (`|PlayMontage` (`self.Mesh`) "/Game/FD10/Characters/MocapOnline/Animations/Fire/A_Pistol_Reload_Montage.A_Pistol_Reload_Montage"
                      (:`then`
                        (set `self.bReloading` true))
                      (:`OnCompleted`
                        (set `self.bReloading` false)))
                    (else
                      (`/Game/FD10/Core/Survival/Items/BP_Weapon.PlayOutOfAmmoSound` (`self.EquippedWeapon`))))))))))
      (else
        (bind (_outhit_hitactor _returnvalue) (`self.HitForInteractableObjects`))
        (if _returnvalue
          (bind _returnvalue_2 (`self.GetComponentByClass` _outhit_hitactor "/Game/FD10/Core/Survival/Components/BP_InteractableComponent.BP_InteractableComponent_C"))
          (`/Engine/EditorBlueprintResources/StandardMacros.IsValid` _returnvalue_2
            (:`Is Valid`
              (`/Game/FD10/Core/Survival/Components/BP_InteractableComponent.OnInteract` _returnvalue_2))))))))

(event `LookAtTarget_Event`
  (params (LookAtLocation :type "Vector Structure") (Duration :type "Float (double-precision)"))
  (`KismetSystemLibrary.K2_ClearAndInvalidateTimerHandle` (`self.LookAtLocationTimer`))
  (set `self.LookAtLocation` LookAtLocation)
  (set `self.bLookingAtLocation` true)
  (bind _returnvalue (`KismetSystemLibrary.K2_SetTimerDelegate` (delegate `CancelLookAtLocation_Event`) Duration))
  (set `self.LookAtLocationTimer` _returnvalue))

(event `CancelLookAtLocation_Event`
  (set `self.bLookingAtLocation` false)
  (`KismetSystemLibrary.K2_ClearAndInvalidateTimerHandle` (`self.LookAtLocationTimer`)))

(fn `EquipWeapon`
  (params (Weapon :type "/Game/FD10/Core/Survival/Items/BP_Weapon Object Reference"))
  (`/Engine/EditorBlueprintResources/StandardMacros.IsValid` (`self.EquippedWeapon`)
    (:`Is Valid`
      (`self.UnequipWeapon`))
    (:`Is Not Valid`
      _))
  (bind _output_get (set `self.EquippedWeapon` Weapon))
  (`self.K2_AttachToComponent` _output_get (`self.Mesh`) (`/Game/FD10/Core/Survival/Items/BP_Weapon.AttachSocket` _output_get) "KeepRelative" "KeepRelative" "KeepRelative" true)
  (`SceneComponent.K2_SetRelativeTransform` (`/Game/FD10/Core/Survival/Items/BP_SurvivalItem.Mesh` (`self.EquippedWeapon`)) (`KismetMathLibrary.MakeTransform` (0.0 0.0 0.0)) false false)
  (`self.SetActorHiddenInGame` (`self.EquippedWeapon`) false))

(fn `UnequipWeapon`
  (`SurvivalItemBase.OnPicked` (`self.EquippedWeapon`))
  (set `self.EquippedWeapon` null))

(fn `UserConstructionScript`)