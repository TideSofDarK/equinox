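; Actor component that makes its owner's point light and mesh material flicker randomly on and off.
; On BeginPlay it swaps the first static mesh material for a dynamic instance and caches its "Intensity" parameter and the light's intensity as base values.
; An endless short random-delay loop scales both by a shared modifier, rerolled to zero or one each pass, keeping light and material in sync.
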(event `self.ReceiveBeginPlay`
  (bind _returnvalue (`self.GetOwner`))
  (set `self.PointLight` (`Actor.GetComponentByClass` _returnvalue "/Script/Engine.PointLightComponent"))
  (set `self.Mesh` (`Actor.GetComponentByClass` _returnvalue "/Script/Engine.StaticMeshComponent"))
  (bind _returnvalue_2 (`KismetMaterialLibrary.CreateDynamicMaterialInstance` (`PrimitiveComponent.GetMaterial` (`self.Mesh`) 0)))
  (bind _output_get (set `self.Material` _returnvalue_2))
  (`PrimitiveComponent.SetMaterial` (`self.Mesh`) 0 _output_get)
  (bind _returnvalue_3 (`MaterialInstanceDynamic.K2_GetScalarParameterValue` (`self.Material`) "Intensity"))
  (set `self.MaterialIntesnity` _returnvalue_3)
  (set `self.LightIntensity` (`LightComponentBase.Intensity` (`self.PointLight`)))
  (`KismetSystemLibrary.RetriggerableDelay` (`KismetMathLibrary.RandomFloatInRange` 0.05 0.25) :!label _label)
  (`MaterialInstanceDynamic.SetScalarParameterValue` (`self.Material`) "Intensity" (* (`self.MaterialIntesnity`) (`self.Modifier`)))
  (`LightComponent.SetIntensity` (`self.PointLight`) (* (`self.LightIntensity`) (`self.Modifier`)))
  (set `self.Modifier` (`KismetMathLibrary.Conv_IntToDouble` (`KismetMathLibrary.Round` (`KismetMathLibrary.RandomFloatInRange` 0.0 1.0))))
  (goto _label))