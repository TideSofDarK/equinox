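; BP_CaptureBox renders a 3D item, mesh or interactive examine scene into a render target and dynamic UI material for the survival UI.
; Init functions scale the content, set up SceneCaptureComponent2D and optionally play a spin-and-scale appear timeline; the actor keeps working while paused.
; Input orbits and zooms the spring-arm camera, while clicks deproject through the capture to reach interactive components.
; Examine targets store camera settings that ZoomTimeline blends between.
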(event `InputAxis|UIZoom` :paused true
  (params (AxisValue :type "Float (single-precision)"))
  (bind _cameraspringarm (`self.CameraSpringArm`))
  (bind _defaultarmlength (`self.DefaultArmLength`))
  (if (`self.CanControlCamera`)
    (set `SpringArmComponent.TargetArmLength` (`KismetMathLibrary.FClamp` (+ (`SpringArmComponent.TargetArmLength` _cameraspringarm) (* AxisValue 50.0 -1.0)) (* _defaultarmlength 0.2) (* _defaultarmlength 1.8)) _cameraspringarm)))

(event `InputAxis|MoveForward/Backwards` :paused true
  (params (AxisValue :type "Float (single-precision)"))
  (if (`self.CanControlCamera`)
    (`SceneComponent.K2_AddRelativeRotation` (`self.CameraSpringArm`) (`KismetMathLibrary.MakeRotator` 0.0 (* AxisValue (`GameplayStatics.GetWorldDeltaSeconds`) (`self.ControlRotationSpeed`) -1.0)) false false)))

(event `InputAxis|MoveRight/Left` :paused true
  (params (AxisValue :type "Float (single-precision)"))
  (if (`self.CanControlCamera`)
    (`SceneComponent.K2_AddRelativeRotation` (`self.CameraSpringArm`) (`KismetMathLibrary.MakeRotator` 0.0 0.0 (* AxisValue (`GameplayStatics.GetWorldDeltaSeconds`) (`self.ControlRotationSpeed`) -1.0)) false false)))

(event `InputAxisKey|MouseX` :paused true
  (params (AxisValue :type "Float (single-precision)"))
  (if (`self.CanControlCamera`)
    (`SceneComponent.K2_AddRelativeRotation` (`self.CameraSpringArm`) (`KismetMathLibrary.MakeRotator` 0.0 0.0 (* AxisValue (`self.ControlMouseRotationSpeed`))) false false)
    (`SceneComponent.K2_SetRelativeRotation` (`self.CameraSpringArm`) (`KismetMathLibrary.MakeRotator` (.roll (`SceneComponent.RelativeRotation` (`self.CameraSpringArm`))) (`KismetMathLibrary.FClamp` (.pitch (`SceneComponent.RelativeRotation` (`self.CameraSpringArm`))) -60.0 60.0) (.yaw (`SceneComponent.RelativeRotation` (`self.CameraSpringArm`)))) false false :!label _label)))

(event `InputAxisKey|MouseY` :paused true
  (params (AxisValue :type "Float (single-precision)"))
  (if (`self.CanControlCamera`)
    (`SceneComponent.K2_AddRelativeRotation` (`self.CameraSpringArm`) (`KismetMathLibrary.MakeRotator` 0.0 (* AxisValue (`self.ControlMouseRotationSpeed`))) false false)
    (goto _label)))

(event `self.ReceiveBeginPlay`
  (`self.SetTickableWhenPaused` true)
  (`ActorComponent.SetTickableWhenPaused` (`self.SceneCaptureComponent2D`) true)
  (`ActorComponent.SetTickableWhenPaused` (`self.AppearTimeline`) true)
  (`ActorComponent.SetTickableWhenPaused` (`self.SkeletalMesh`) true)
  (`ActorComponent.SetTickableWhenPaused` (`self.CameraSpringArm`) true)
  (`ActorComponent.SetTickableWhenPaused` (`self.InteractiveSceneRoot`) true)
  (`ActorComponent.SetTickableWhenPaused` (`self.ZoomTimeline`) true)
  (`SurvivalPlayerController.HideActor` (cast `SurvivalPlayerController` (`GameplayStatics.GetPlayerController` 0) :!pure true) self)
  (`self.SetActorEnableCollision` false)
  (set `self.ZoomedExamineTarget` (`self.RootExamineTarget`)))

(event `self.ReceiveTick`
  (params (DeltaSeconds :type "Float (single-precision)"))
  (if (`self.bAlwaysCaptureScene`)
    (`|ExecutionSequence`
      (:`then_0`
        (if (and (not (`TimelineComponent.IsPlaying` (`self.AppearTimeline`))) (`self.bConstantRotation`))
          (`SceneComponent.K2_AddRelativeRotation` (`self.InteractiveSceneRoot`) (`KismetMathLibrary.MakeRotator` 0.0 0.0 (* DeltaSeconds 75.0)) false false)))
      (:`then_1`
        (`SceneCaptureComponent2D.CaptureScene` (`self.SceneCaptureComponent2D`))))))

(event `OnComponentClicked_Event`
  (params (ClickedComponent :type "PrimitiveComponent Object Reference")))

(event `Key|LeftMouseButton` :paused true
  (params (Key :type "Key Structure"))
  (:`Pressed`
    (if (`self.bControlsEnabled`)
      (bind (_outhit _returnvalue) (`self.ProjectClick`))
      (if _returnvalue
        (if (== (`.HitActor` (`GameplayStatics.BreakHitResult` _outhit)) self)
          (bind _asinteractive_static_mesh_component (cast `InteractiveStaticMeshComponent` (`.HitComponent` (`GameplayStatics.BreakHitResult` _outhit))))
          (if (`InteractiveStaticMeshComponent.bCanBeClicked` _asinteractive_static_mesh_component)
            (`InteractiveStaticMeshComponent.DispatchOnClickedBlueprint` _asinteractive_static_mesh_component Key)))))))

(event `CaptureOnceWithDelay`
  (`KismetSystemLibrary.Delay` 0.05)
  (`SceneCaptureComponent2D.CaptureScene` (`self.SceneCaptureComponent2D`)))

(event `Key|RightMouseButton` :paused true
  (params (Key :type "Key Structure"))
  (:`Pressed`
    (`self.Unzoom_Event` :!label _label_2)))

(event `InputAction|UIDecline` :paused true
  (params (Key :type "Key Structure"))
  (:`Pressed`
    (goto _label_2)))

(event `Unzoom_Event`
  (if (and (`self.bControlsEnabled`) (not (`TimelineComponent.IsPlaying` (`self.ZoomTimeline`))))
    (if (== (`self.RootExamineTarget`) (`self.ZoomedExamineTarget`))
      (`self.CloseED` :!label _label_3)
      (set `self.bControlsEnabled` false)
      (set `self.bCameraControlsEnabled` false)
      (else
        (bind _asbp_examine_target (cast `/Game/FD10/Core/Survival/Items/BP_ExamineTarget` (`SceneComponent.GetAttachParent` (`self.ZoomedExamineTarget`))))
        (`self.ZoomIntoExamineTarget_Event` _asbp_examine_target)))))

(event `InputAction|Inventory` :paused true
  (params (Key :type "Key Structure"))
  (:`Pressed`
    (if (and (`self.bControlsEnabled`) (not (`TimelineComponent.IsPlaying` (`self.ZoomTimeline`))))
      (goto _label_3))))

(event `ZoomIntoExamineTarget_Event`
  (params (ExamineTarget :type "/Game/FD10/Core/Survival/Items/BP_ExamineTarget Object Reference") (Delay :type "Float (double-precision)"))
  (set `/Game/FD10/Core/Survival/Items/BP_ExamineTarget.bZoomedIn` false (`self.ZoomedExamineTarget`))
  (`/Game/FD10/Core/Survival/Items/BP_ExamineTarget.OnZoomed` (`self.ZoomedExamineTarget`) false)
  (bind _output_get (set `self.PreviousExamineTarget` (`self.ZoomedExamineTarget`)))
  (`/Game/FD10/Core/Survival/Items/BP_ExamineTarget.DumpCameraSettings` _output_get (`self.CameraSpringArm`))
  (bind _output_get_2 (set `self.ZoomedExamineTarget` ExamineTarget))
  (if (not (`/Game/FD10/Core/Survival/Items/BP_ExamineTarget.bInitializedDumpValues` _output_get_2))
    (`/Game/FD10/Core/Survival/Items/BP_ExamineTarget.InitializeDumpValues` (`self.ZoomedExamineTarget`)))
  (set `/Game/FD10/Core/Survival/Items/BP_ExamineTarget.bZoomedIn` true (`self.ZoomedExamineTarget`))
  (set `self.bControlsEnabled` false)
  (set `self.bCameraControlsEnabled` false)
  (`KismetSystemLibrary.Delay` Delay)
  (`TimelineComponent.PlayFromStart` (`self.ZoomTimeline`)))

(fn `CalculateAndApplyScale`
  (params (MaxExtent :type "Float (double-precision)"))
  (bind (_origin _boxextent) (`KismetSystemLibrary.GetComponentBounds` (`self.SkeletalMesh`)))
  (`SceneComponent.SetRelativeScale3D` (`self.InteractiveSceneRoot`) (/ (* (`self.GetActorScale3D`) (/ MaxExtent (+ (`KismetMathLibrary.FMax` (.y _boxextent) (.z _boxextent)) (.x _boxextent)))) 2.0)))

(fn `DestroyAndCleanup`
  (`KismetRenderingLibrary.ReleaseRenderTarget2D` (`self.RenderTarget`))
  (set `self.MaterialInstance` null)
  (if (`self.bDontDestroyScene`)
    (`self.SetActorTickEnabled` false)
    (`self.SetActorEnableCollision` false)
    (else
      (`self.K2_DestroyActor`))))

(fn `InitializeInteractiveScene`
  (params (ExtentScale :type "Float (double-precision)"))
  (returns (MaterialInstance :type "MaterialInstance Object Reference") (RenderTarget :type "TextureRenderTarget Object Reference") (InteractiveScene :type "/Game/FD10/Core/Survival/Items/BP_CaptureBox Object Reference"))
  (`self.SetActorEnableCollision` true)
  (bind (_materialinstance _rendertarget) (`self.InitializeInternal` (struct) true 1 true ExtentScale))
  (return _materialinstance _rendertarget self))

(fn `InitializeInternal`
  (params (MeshRotation :type "Rotator Structure") (PlayAppearAnimation :type Boolean) (RenderTargetResolutionScale :type Integer :default 1) (bFullScreen :type Boolean) (ExtentScale :type "Float (double-precision)" :default 1.0))
  (returns (MaterialInstance :type "MaterialInstance Object Reference") (RenderTarget :type "TextureRenderTarget Object Reference"))
  (bind (_returnvalue_x _returnvalue_y) (`KismetMathLibrary.BreakVector2D` (`WidgetLayoutLibrary.GetViewportSize`)))
  (bind _fullscreendownscalefactor (`self.FullScreenDownscaleFactor`))
  (bind _returnvalue (/ _returnvalue_y _returnvalue_x))
  (bind _returnvalue_2 (* (`local.RenderTargetResolutionScale`) 128))
  (`self.SetActorTickEnabled` true)
  (`self.ResetSpringArmLength`)
  (`SceneCaptureComponent.ShowOnlyActorComponents` (`self.SceneCaptureComponent2D`) self)
  (`self.CalculateAndApplyScale` (`self.MaxExtent`))
  (`SceneComponent.K2_SetRelativeRotation` (`self.SkeletalMesh`) (`local.MeshRotation`) false false)
  (if (`local.bFullScreen`)
    (bind _returnvalue_3 (`KismetRenderingLibrary.CreateRenderTarget2D` (/ (`KismetMathLibrary.FTrunc` _returnvalue_x) _fullscreendownscalefactor) (/ (`KismetMathLibrary.FTrunc` _returnvalue_y) _fullscreendownscalefactor) "RTF_RGBA8"))
    (set `self.RenderTarget` _returnvalue_3)
    (`SceneComponent.SetRelativeScale3D` (`self.InteractiveSceneRoot`) (* (`SceneComponent.RelativeScale3D` (`self.InteractiveSceneRoot`)) (`KismetMathLibrary.MakeVector` _returnvalue _returnvalue _returnvalue)))
    (else
      (bind _returnvalue_4 (`KismetRenderingLibrary.CreateRenderTarget2D` _returnvalue_2 _returnvalue_2 "RTF_RGBA8"))
      (set `self.RenderTarget` _returnvalue_4)))
  (set `Texture.Filter` "TF_Nearest" (`self.RenderTarget`))
  (bind _returnvalue_5 (`KismetMaterialLibrary.CreateDynamicMaterialInstance` "/Game/FD10/MaterialLibrary/M_SceneCapture_UI.M_SceneCapture_UI"))
  (bind _output_get (set `self.MaterialInstance` _returnvalue_5))
  (`MaterialInstanceDynamic.SetTextureParameterValue` _output_get "Texture" (`self.RenderTarget`))
  (set `SceneCaptureComponent2D.TextureTarget` (`self.RenderTarget`) (`self.SceneCaptureComponent2D`))
  (if (`local.PlayAppearAnimation`)
    (`self.PlayAppearAnimation` true))
  (set `self.bInitialized` true)
  (`self.CaptureOnceWithDelay`)
  (return (`self.MaterialInstance`) (`self.RenderTarget`)))

(fn `InitializeItemVisual`
  (params (PlayAppearAnimation :type Boolean) (Item :type "/Game/FD10/Core/Survival/Items/BP_Item_Survival Object Reference"))
  (returns (MaterialInstance :type "MaterialInstance Object Reference") (RenderTarget :type "TextureRenderTarget Object Reference"))
  (bind _item (`local.Item`))
  (bind (_x _y) (break `IntVector` (`/Game/FD10/Core/Survival/Items/BP_Item_Survival.InventorySize` (`local.Item`))))
  (`SkinnedMeshComponent.SetSkinnedAssetAndUpdate` (`self.SkeletalMesh`) (`/Game/FD10/Core/Survival/Items/BP_Item_Survival.DefaultMesh` _item) true)
  (bind (_materialinstance _rendertarget) (`self.InitializeInternal` (`/Game/FD10/Core/Survival/Items/BP_Item_Survival.Inventory3DRotation` _item) PlayAppearAnimation (`KismetMathLibrary.Max` _x _y)))
  (return _materialinstance _rendertarget))

(fn `InitializeVisual`
  (params (Mesh :type "SkeletalMesh Object Reference") (MeshRotation :type "Rotator Structure") (PlayAppearAnimation :type Boolean) (RenderTargetResolutionScale :type Integer) (bFullScreen :type Boolean) (bEnableCollision :type Boolean))
  (returns (MaterialInstance :type "MaterialInstance Object Reference") (RenderTarget :type "TextureRenderTarget Object Reference"))
  (`self.SetActorEnableCollision` bEnableCollision)
  (`SkinnedMeshComponent.SetSkinnedAssetAndUpdate` (`self.SkeletalMesh`) Mesh true)
  (bind (_materialinstance _rendertarget) (`self.InitializeInternal` (`local.MeshRotation`) (`local.PlayAppearAnimation`) (`local.RenderTargetResolutionScale`) bFullScreen))
  (return _materialinstance _rendertarget))

(fn `PlayAppearAnimation`
  (params (bIn :type Boolean))
  (bind _appeartimeline (`self.AppearTimeline`))
  (if bIn
    (`TimelineComponent.PlayFromStart` _appeartimeline)
    (else
      (`TimelineComponent.ReverseFromEnd` _appeartimeline))))

(fn `ProjectClick`
  (returns (OutHit :type "HitResult Structure") (ReturnValue :type Boolean))
  (bind (_locationx _locationy) (`PlayerController.GetMousePosition` (`GameplayStatics.GetPlayerController` 0)))
  (bind (_outworldorigin _outworlddirection) (`GameplayUtilities.CaptureComponent2D_DeProject` (`self.SceneCaptureComponent2D`) (`KismetMathLibrary.MakeVector2D` _locationx _locationy)))
  (bind (_outhit _returnvalue) (`KismetSystemLibrary.LineTraceSingleForObjects` :`Start` _outworldorigin :`End` (+ _outworldorigin (* _outworlddirection 1000.0)) :`ObjectTypes` (`|MakeArray` "ObjectTypeQuery8" :!type "EObjectTypeQuery Enum") :`bIgnoreSelf` false :`DrawTime` 100.0))
  (return _outhit _returnvalue))

(fn `ResetInitialVisualState`
  (`SceneComponent.K2_SetRelativeRotation` :`self` (`self.InteractiveSceneRoot`))
  (`SceneCaptureComponent2D.CaptureScene` (`self.SceneCaptureComponent2D`)))

(fn `ResetSpringArmLength`
  (set `SpringArmComponent.TargetArmLength` (`self.DefaultArmLength`) (`self.CameraSpringArm`)))

(fn `ResetTransforms`
  (`SceneComponent.ResetRelativeTransform` (`self.InteractiveSceneRoot`))
  (`SceneComponent.ResetRelativeTransform` (`self.CameraSpringArm`))
  (`SceneComponent.ResetRelativeTransform` (`self.AppearAnimationRoot`)))

(fn `UserConstructionScript`
  (`self.ResetSpringArmLength`))