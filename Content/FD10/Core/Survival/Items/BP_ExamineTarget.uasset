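; BP_ExamineTarget is a scene component for survival items that marks a point the camera examines and signals when it is examined.
; Examine fires the OnExamined dispatcher.
; InitializeDumpValues seeds stored camera location, rotation and distance from the component's world location, reversed forward vector and CameraDistance.
; DumpCameraSettings overwrites those values from a supplied spring arm's world location, relative rotation and arm length.
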(event `self.ReceiveBeginPlay`)

(fn `DumpCameraSettings`
  (params (SpringArm :type "SpringArmComponent Object Reference"))
  (set `self.DumpedLocation` (`self.K2_GetComponentLocation` SpringArm))
  (set `self.DumpedRotation` (`SceneComponent.RelativeRotation` SpringArm))
  (set `self.DumpedDistance` (`SpringArmComponent.TargetArmLength` SpringArm)))

(fn `Examine`
  (`self.OnExamined`))

(fn `InitializeDumpValues`
  (set `self.DumpedDistance` (`self.CameraDistance`))
  (set `self.DumpedRotation` (`KismetMathLibrary.Conv_VectorToRotator` (* (`self.GetForwardVector`) -1.0)))
  (set `self.DumpedLocation` (`self.K2_GetComponentLocation`))
  (set `self.bInitializedDumpValues` true))