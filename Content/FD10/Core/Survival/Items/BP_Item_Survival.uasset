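; Base survival item actor that the player picks up through an interactable component and keeps in an inventory.
; Interaction notifies the survival player controller; post-pickup hides the actor, disables collision and removes its particle effect.
; Combine merges stack counts of same-class stackable items, while helpers swap grid dimensions and derive widget render scale.
; It also spawns and caches an interactive item scene actor, with Use left empty.
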(event `self.ReceiveBeginPlay`
  (add `/Game/FD10/Core/Components/BP_InteractableComponent.InteractableED` (`self.BP_InteractableComponent`) (delegate `OnPickup_Event`)))

(event `OnPickup_Event`
  (bind _asbp_player_controller_survival (cast `/Game/FD10/Core/BP_PlayerController_Survival` (`GameplayStatics.GetPlayerController` 0)))
  (`/Game/FD10/Core/BP_PlayerController_Survival.OnItemPickup_Event` _asbp_player_controller_survival self))

(event `OnPostPickup_Event`
  (`PrimitiveComponent.SetCollisionEnabled` (`self.Mesh`) "NoCollision")
  (`self.SetActorHiddenInGame` true)
  (`ActorComponent.K2_DestroyComponent` (`self.ParticleSystem`))
  (`self.K2_SetActorTransform` (`KismetMathLibrary.MakeTransform` (0.0 0.0 0.0))))

(fn `Combine`
  (params (OtherItem :type "/Game/FD10/Core/Survival/Items/BP_Item_Survival Object Reference"))
  (returns (Result :type "/Game/FD10/Core/Survival/Items/ECombineResult Enum") (NewItem :type "/Game/FD10/Core/Survival/Items/BP_Item_Survival Object Reference"))
  (bind _combinesound (`self.CombineSound`))
  (bind _returnvalue (select `bool` (and (== (`GameplayStatics.GetObjectClass` self) (`GameplayStatics.GetObjectClass` OtherItem)) (`self.bCanBeStacked`) (!= (`local.OtherItem`) self)) :`false` "NewEnumerator2" :`true` "NewEnumerator0" :!type "/Game/FD10/Core/Survival/Items/ECombineResult Enum"))
  (if (`|EnumEquality` _returnvalue "NewEnumerator0")
    (set `self.StackCount` (+ (`/Game/FD10/Core/Survival/Items/BP_Item_Survival.StackCount` (`local.OtherItem`)) (`self.StackCount`)))
    (`/Engine/EditorBlueprintResources/StandardMacros.IsValid` _combinesound
      (:`Is Valid`
        (`GameplayStatics.PlaySound2D` _combinesound 1.0 1.0 0.0 null null))
      (:`Is Not Valid`
        _)))
  (return _returnvalue null))

(fn `GetDefaultWidgetRenderScale`
  (returns (ReturnValue :type "Float (double-precision)"))
  (bind (_x _y) (break `IntVector` (`self.InventorySize`)))
  (return (* (`KismetMathLibrary.Max` _x _y) (`self.InventoryScale`))))

(fn `GetInteractiveItemScene`
  (params (bRecreate :type Boolean))
  (returns (Output_Get :type "/Game/FD10/Core/Survival/Items/BP_CaptureBox Object Reference"))
  (`/Engine/EditorBlueprintResources/StandardMacros.IsValid` (`self.InteractiveItemScene`)
    (:`Is Valid`
      (if (`local.bRecreate`)
        (`self.K2_DestroyActor` (`self.InteractiveItemScene`))
        (bind _returnvalue (`|SpawnActorFromClass` (`self.InteractiveItemSceneClass`) (`KismetMathLibrary.MakeTransform` (0.0 0.0 0.0)) "Undefined" "OverrideRootScale" null self null :!label _label))
        (bind _output_get (set `self.InteractiveItemScene` _returnvalue))
        (set `/Game/FD10/Core/Survival/Items/BP_CaptureBox.bDontDestroyScene` true _output_get)))
    (:`Is Not Valid`
      (goto _label)))
  (return (`self.InteractiveItemScene`)))

(fn `HasUniqueInteractiveItemScene`
  (returns (bHasUniqueInteractiveItemScene :type Boolean))
  (bind _interactiveitemsceneclass (`self.InteractiveItemSceneClass`))
  (return (and (!= _interactiveitemsceneclass "/Game/FD10/Core/Survival/Items/BP_CaptureBox.BP_CaptureBox_C") (`KismetSystemLibrary.IsValidClass` _interactiveitemsceneclass))))

(fn `SwapInventoryWidthAndHeight`
  (locals (OldInventorySize :type "IntVector Structure"))
  (bind _output_get (set `local.OldInventorySize` (`self.InventorySize`)))
  (set `self.InventorySize` (make `IntVector` (`.Y` (break `IntVector` _output_get)) (break `IntVector` _output_get))))

(fn `Use`)

(fn `UserConstructionScript`
  (`SkinnedMeshComponent.SetSkinnedAssetAndUpdate` (`self.Mesh`) (`self.DefaultMesh`) true)
  (`SceneComponent.SetWorldScale3D` (`self.ParticleSystem`) (1.0 1.0 1.0)))