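; Weapon item for the survival game that toggles equip from Use and treats its stack count as loaded ammo.
; Fire spends ammo and calls TraceShot, while Reload refills from matching ammo items in the inventory grid, removing emptied stacks.
; TraceShot box-traces physics bodies to damage characters and trigger hit reactions, falling back to a line trace for decals when none is found, with surface-based impact effects and sounds.
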(event `self.Use`
  (bind _asbp_survival_main_character (cast `/Game/FD10/Core/Survival/Characters/BP_SurvivalMainCharacter` (`GameplayStatics.GetPlayerCharacter` 0)))
  (bind _equippedweapon (`/Game/FD10/Core/Survival/Characters/BP_SurvivalMainCharacter.EquippedWeapon` _asbp_survival_main_character)
    (:`then`
      (if (== _equippedweapon self)
        (`/Game/FD10/Core/Survival/Characters/BP_SurvivalMainCharacter.UnequipWeapon` _asbp_survival_main_character)
        (set `self.UseCaption` (defaults `/Game/FD10/Core/Survival/Items/BP_Weapon` "BP_Weapon_C"))))
    (:`else`
      (`/Game/FD10/Core/Survival/Characters/BP_SurvivalMainCharacter.EquipWeapon` _asbp_survival_main_character self)
      (`GameplayStatics.PlaySound2D` (`self.EquipSound`) 1.0 1.0 0.0 null null)
      (set `self.UseCaption` "Unequip"))))

(fn `Combine`
  (params (OtherItem :type "/Game/FD10/Core/Survival/Items/BP_SurvivalItem Object Reference"))
  (returns (Result :type "/Game/FD10/Core/Survival/Items/ECombineResult Enum") (NewItem :type "/Game/FD10/Core/Survival/Items/BP_SurvivalItem Object Reference"))
  (return "NewEnumerator2" null))

(fn `Fire`
  (returns (bSuccess :type Boolean))
  (bind _fireorigin (`self.FireOrigin`))
  (if (`self.IsEnoughAmmo`)
    (set `self.StackCount` (- (`self.StackCount`) (`self.FireCost`)))
    (`self.TraceShot` (`SceneComponent.K2_GetComponentLocation` _fireorigin) (`SceneComponent.GetForwardVector` _fireorigin) 1000.0 (`self.Damage`))
    (return true)
    (else
      (return false))))

(fn `IsEnoughAmmo`
  (returns (ReturnValue :type Boolean))
  (return (>= (`self.StackCount`) (`self.FireCost`))))

(fn `PlayOutOfAmmoSound`
  (`GameplayStatics.PlaySoundAtLocation` (`self.OutOfAmmoSound`) (`self.K2_GetActorLocation`) (struct) 1.0 1.0 0.0 null null null))

(fn `Reload`
  (params (InventoryGrid :type "Map of IntVector Structure to /Game/FD10/Core/Survival/Items/BP_SurvivalItem Object Reference (by ref)"))
  (returns (bAtleastOneBullet :type Boolean))
  (locals (CounterLocal :type Integer) (bAtleastOneBulletLocal :type Boolean) (SubCounterLocal :type Integer))
  (bind _counterlocal (`local.CounterLocal`))
  (bind _keys (`BlueprintMapLibrary.Map_Keys` InventoryGrid))
  (set `local.CounterLocal` (- (`self.MaxStackCount`) (`self.StackCount`)))
  (for _array_element _keys
    (bind _value (`BlueprintMapLibrary.Map_Find` InventoryGrid _array_element))
    (if (== (`GameplayStatics.GetObjectClass` _value) (`self.AmmoClass`))
      (set `local.bAtleastOneBulletLocal` true)
      (bind _stackcount (`/Game/FD10/Core/Survival/Items/BP_SurvivalItem.StackCount` _value))
      (if (<= _stackcount _counterlocal)
        (set `local.CounterLocal` (- _counterlocal _stackcount))
        (`self.K2_DestroyActor` _value)
        (`BlueprintMapLibrary.Map_Remove` (`local.InventoryGrid`) _array_element)
        (else
          (set `/Game/FD10/Core/Survival/Items/BP_SurvivalItem.StackCount` (- _stackcount _counterlocal) _value)
          (set `local.CounterLocal` 0)))
      (if (== (`local.CounterLocal`) 0)
        (break))))
  (set `self.StackCount` (- (`self.MaxStackCount`) (`local.CounterLocal`)))
  (return (`local.bAtleastOneBulletLocal`)))

(fn `TraceShot`
  (params (Start :type "Vector Structure") (Direction :type "Vector Structure") (Length :type "Float (double-precision)") (Damage :type "Float (double-precision)"))
  (returns (bHit :type Boolean) (HitActor :type "Actor Object Reference"))
  (locals (CachedCharacter :type "SurvivalCharacterBase Object Reference"))
  (bind _returnvalue (+ Start (* Direction Length)))
  (bind (_outhit _returnvalue_2) (`KismetSystemLibrary.BoxTraceSingleForObjects` (`local.Start`) _returnvalue (50.0 50.0 50.0) (struct) (`|MakeArray` "ObjectTypeQuery4" :!type "EObjectTypeQuery Enum") false (`|MakeArray` (`self.GetOwner`)) "None" true (struct :`R` 1.0 :`A` 1.0) (struct :`G` 1.0 :`A` 1.0) 1.0))
  (if _returnvalue_2
    (bind _assurvival_character_base (cast `SurvivalCharacterBase` (`.HitActor` (`GameplayStatics.BreakHitResult` _outhit)))
      (:`then`
        (bind _output_get (set `local.CachedCharacter` _assurvival_character_base))
        (`GameplayStatics.ApplyDamage` _output_get (`self.Damage`))
        (bind _surfacetype (`PhysicalMaterial.SurfaceType` (`.PhysMat` (`GameplayStatics.BreakHitResult` _outhit))))
        (bind (_returnvalue_roll _returnvalue_pitch _returnvalue_yaw) (`KismetMathLibrary.BreakRotator` (`KismetMathLibrary.NormalizedDeltaRotator` (`KismetMathLibrary.Conv_VectorToRotator` (`.ImpactNormal` (`GameplayStatics.BreakHitResult` _outhit))) (`KismetMathLibrary.Conv_VectorToRotator` (`local.Direction`)))))
        (`NiagaraFunctionLibrary.SpawnSystemAttached` (`/Game/FD10/Environment/BulletImpact/BPFL_BulletImpact.BulletImpactFX` _surfacetype) (`.HitComponent` (`GameplayStatics.BreakHitResult` _outhit)) "None" (`.ImpactPoint` (`GameplayStatics.BreakHitResult` _outhit)) (`KismetMathLibrary.Conv_VectorToRotator` (`KismetMathLibrary.RotateAngleAxis` (`.ImpactNormal` (`GameplayStatics.BreakHitResult` _outhit)) (* (- 180.0 _returnvalue_yaw) -1.0) (0.0 0.0 1.0))) "KeepWorldPosition")
        (`GameplayStatics.PlaySoundAtLocation` (`/Game/FD10/Environment/BulletImpact/BPFL_BulletImpact.BulletImpactSound` _surfacetype) (`.ImpactPoint` (`GameplayStatics.BreakHitResult` _outhit)) (struct) 1.0 1.0 0.0 null null null)
        (message `/Game/FD10/Core/Survival/Characters/BPI_HitReaction.HitReaction` (`local.CachedCharacter`) (`.HitBoneName` (`GameplayStatics.BreakHitResult` _outhit)) (`KismetMathLibrary.Normal` (- (`.ImpactPoint` (`GameplayStatics.BreakHitResult` _outhit)) (`local.Start`))))
        (return true (`local.CachedCharacter`)))
      (:`CastFailed`
        (return false null)))
    (else
      (bind (_outhit_2 _returnvalue_3) (`KismetSystemLibrary.LineTraceSingleForObjects` :`Start` (`local.Start`) :`End` _returnvalue :`ObjectTypes` (`|MakeArray` "ObjectTypeQuery3" "ObjectTypeQuery1" :!type "EObjectTypeQuery Enum") :`DrawTime` 1.0))
      (`/Engine/EditorBlueprintResources/StandardMacros.IsValid` (`.PhysMat` (`GameplayStatics.BreakHitResult` _outhit_2))
        (:`Is Valid`
          (bind _surfacetype_2 (`PhysicalMaterial.SurfaceType` (`.PhysMat` (`GameplayStatics.BreakHitResult` _outhit_2))))
          (bind _returnvalue_4 (`GameplayStatics.SpawnDecalAtLocation` (`/Game/FD10/Environment/BulletImpact/BPFL_BulletImpact.RandomBulletDecal` _surfacetype_2) (5.0 10.0 10.0) (`.ImpactPoint` (`GameplayStatics.BreakHitResult` _outhit_2)) (`KismetMathLibrary.Conv_VectorToRotator` (* (`.ImpactNormal` (`GameplayStatics.BreakHitResult` _outhit_2)) -1.0))))
          (`DecalComponent.SetFadeScreenSize` _returnvalue_4 0.0)
          (`SceneComponent.K2_AttachToComponent` _returnvalue_4 (`.HitComponent` (`GameplayStatics.BreakHitResult` _outhit_2)) (`.HitBoneName` (`GameplayStatics.BreakHitResult` _outhit_2)) "KeepWorld" "KeepWorld" "KeepWorld" true)
          (`|ExecutionSequence`
            (:`then_0`
              (`GameplayStatics.PlaySoundAtLocation` (`/Game/FD10/Environment/BulletImpact/BPFL_BulletImpact.BulletImpactSound` _surfacetype_2) (`.ImpactPoint` (`GameplayStatics.BreakHitResult` _outhit_2)) (struct) 1.0 1.0 0.0 null null null))
            (:`then_1`
              (bind (_returnvalue_roll_2 _returnvalue_pitch_2 _returnvalue_yaw_2) (`KismetMathLibrary.BreakRotator` (`KismetMathLibrary.NormalizedDeltaRotator` (`KismetMathLibrary.Conv_VectorToRotator` (`.ImpactNormal` (`GameplayStatics.BreakHitResult` _outhit_2))) (`KismetMathLibrary.Conv_VectorToRotator` (`local.Direction`)))))
              (`NiagaraFunctionLibrary.SpawnSystemAttached` (`/Game/FD10/Environment/BulletImpact/BPFL_BulletImpact.BulletImpactFX` _surfacetype_2) (`.HitComponent` (`GameplayStatics.BreakHitResult` _outhit_2)) "None" (`.ImpactPoint` (`GameplayStatics.BreakHitResult` _outhit_2)) (`KismetMathLibrary.Conv_VectorToRotator` (`KismetMathLibrary.RotateAngleAxis` (`.ImpactNormal` (`GameplayStatics.BreakHitResult` _outhit_2)) (* (- 180.0 _returnvalue_yaw_2) -1.0) (0.0 0.0 1.0))) "KeepWorldPosition"))
            (:`then_2`
              (return _returnvalue_3 (`.HitActor` (`GameplayStatics.BreakHitResult` _outhit_2))))))
        (:`Is Not Valid`
          (return _returnvalue_3 (`.HitActor` (`GameplayStatics.BreakHitResult` _outhit_2))))))))

(fn `UserConstructionScript`
  (`parent.UserConstructionScript`))