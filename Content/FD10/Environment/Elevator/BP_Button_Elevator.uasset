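; BP_Button_Elevator is an elevator button actor that shows whether it can be interacted with.
; SetState stores the state, swaps the mesh between green and red materials, toggles matching point lights and sets the interactable component's availability.
; The construction script reapplies State, so placed buttons preview their look in the editor.
; PlayButtonSound plays a click at the green light's location.
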(event `SetState`
  (params (NewState :type Boolean))
  (set `self.bState` NewState)
  (`PrimitiveComponent.SetMaterial` (`self.StaticMesh`) 0 (select `bool` NewState :`false` "/Game/FD10/Environment/Elevator/MI_ElevatorButtonR.MI_ElevatorButtonR" :`true` "/Game/FD10/Environment/Elevator/MI_ElevatorButtonG.MI_ElevatorButtonG" :!type "MaterialInterface Object Reference"))
  (`SceneComponent.SetVisibility` (`self.PointLightG`) NewState false)
  (`SceneComponent.SetVisibility` (`self.PointLightR`) (not NewState) false)
  (set `/Game/FD10/Core/Survival/Components/BP_InteractableComponent.bAvailableForInteract` NewState (`self.BP_InteractableComponent`)))

(event `PlayButtonSound`
  (`GameplayStatics.PlaySoundAtLocation` "/Game/FD10/Environment/Elevator/A_ElevatorButtonClick.A_ElevatorButtonClick" (`SceneComponent.K2_GetComponentLocation` (`self.PointLightG`)) (struct) 1.0 1.0 0.1 null null null))

(fn `UserConstructionScript`
  (`parent.UserConstructionScript`)
  (`self.SetState` (`self.bState`)))