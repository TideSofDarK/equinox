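; Elevator actor that travels between its starting location and a Target actor when its linked button is interacted with.
; Activate ignores presses while the elevator or origin gate is moving, otherwise toggles the current end's gate and the button.
; The gate's event dispatcher then triggers Lift, which plays movement audio and runs a timeline forward or in reverse to lerp position.
; On finish, State flips, so CurrentGate selects the arrival gate to toggle.
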(event `self.ReceiveBeginPlay`
  (set `self.Origin` (`self.K2_GetActorLocation`))
  (add `/Game/FD10/Core/Survival/Actors/BP_InteractableActor.OnInteracted` (`self.Button`) (delegate `Activate`)))

(event `Activate`
  (bind _returnvalue (`self.CurrentGate`))
  (bind _button (`self.Button`))
  (if (and (not (`self.bMoving`)) (not (`/Game/FD10/Environment/Elevator/BP_ElevatorGate.bMoving` (`self.GateOrigin`))))
    (`/Game/FD10/Environment/Elevator/BP_ElevatorGate.ForceToggle` _returnvalue)
    (add `/Game/FD10/Environment/Elevator/BP_ElevatorGate.GateED` _returnvalue (delegate `Lift`))
    (`/Game/FD10/Environment/Elevator/BP_Button_Elevator.SetState` _button (not (`/Game/FD10/Environment/Elevator/BP_Button_Elevator.bState` _button)))
    (set `self.bMoving` true)
    (`/Game/FD10/Environment/Elevator/BP_Button_Elevator.PlayButtonSound` (`self.Button`))))

(event `Lift`
  (clear `/Game/FD10/Environment/Elevator/BP_ElevatorGate.GateED` (`self.CurrentGate`))
  (`AudioComponent.Play` (`self.A_ElevatorMovement`) 0.0)
  (if (`self.bState`)
    (bind (_direction _z) (`Timeline|ElevatorTimeline` :!via `ReverseFromEnd` :!label _label)
      (:`Update`
        (`self.K2_SetActorLocation` (`KismetMathLibrary.VLerp` (`self.Origin`) (`self.K2_GetActorLocation` (`self.Target`)) _z)))
      (:`Finished`
        (set `self.bMoving` false)
        (set `self.bState` (not (`self.bState`)))
        (`/Game/FD10/Environment/Elevator/BP_ElevatorGate.ForceToggle` (`self.CurrentGate`))))
    (else
      (goto _label :!via `PlayFromStart`))))

(fn `UserConstructionScript`)