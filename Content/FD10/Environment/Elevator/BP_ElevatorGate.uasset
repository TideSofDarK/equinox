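; Elevator gate that slides two panels open and shut with sound, triggered by its button or by ForceToggle, which skips the button checks.
; Each toggle flips the button state and box collision, then plays or reverses one timeline that mirrors the panels along Y.
; When movement finishes, a closed gate fires the GateED dispatcher, while an open one enables the elevator's button and plays a notify sound.
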(event `self.ReceiveBeginPlay`
  (add `/Game/FD10/Core/Survival/BP_Button.ButtonED` (`self.Button`) (delegate `Toggle`))
  (`PrimitiveComponent.SetCollisionEnabled` (`self.Box`) "NoCollision"))

(event `ForceToggle`
  (bind _gater (`self.GateR`))
  (bind _button (`self.Button`))
  (bind (_relativelocation_x _relativelocation_y _relativelocation_z) (`KismetMathLibrary.BreakVector` (`SceneComponent.RelativeLocation` _gater)))
  (`GameplayStatics.PlaySoundAtLocation` "/Game/FD10/Environment/Elevator/A_ElevatorGate_Cue.A_ElevatorGate_Cue" (`self.K2_GetActorLocation`) (struct) 1.0 1.0 0.0 null null null :!label _label)
  (set `self.bMoving` true)
  (`/Game/FD10/Environment/Elevator/BP_Button_Elevator.SetState` _button (not (`/Game/FD10/Environment/Elevator/BP_Button_Elevator.bState` _button)))
  (`PrimitiveComponent.SetCollisionEnabled` (`self.Box`) (select `bool` (`self.bClosed`) :`false` "QueryAndPhysics" :`true` "NoCollision" :!type "ECollisionEnabled Enum"))
  (if (`self.bClosed`)
    (bind (_direction _y) (`Timeline|GateTimeline` :!label _label_2)
      (:`Update`
        (`SceneComponent.K2_SetRelativeLocation` (`self.GateL`) (`KismetMathLibrary.MakeVector` 0.0 _y) false false)
        (`SceneComponent.K2_SetRelativeLocation` _gater (`KismetMathLibrary.MakeVector` _relativelocation_x (- 0.0 _y) _relativelocation_z) false false))
      (:`Finished`
        (set `self.bClosed` (not (`self.bClosed`)))
        (set `self.bMoving` false)
        (if (`self.bClosed`)
          (`self.GateED`)
          (else
            (`/Game/FD10/Environment/Elevator/BP_Button_Elevator.SetState` (`/Game/FD10/Environment/Elevator/BP_Elevator.Button` (`self.Elevator`)) true)
            (`GameplayStatics.PlaySoundAtLocation` "/Game/FD10/Environment/Elevator/A_ElevatorNotify.A_ElevatorNotify" (`self.K2_GetActorLocation`) (struct) 0.7 1.0 0.0 null null null)))))
    (else
      (goto _label_2 :!via `Reverse`))))

(event `Toggle`
  (if (not (or (`self.bMoving`) (not (`/Game/FD10/Environment/Elevator/BP_Button_Elevator.bState` (`self.Button`)))))
    (`/Game/FD10/Environment/Elevator/BP_Button_Elevator.PlayButtonSound` (`self.Button`))
    (goto _label)))

(fn `UserConstructionScript`)