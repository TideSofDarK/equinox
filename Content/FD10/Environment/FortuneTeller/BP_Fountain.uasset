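; BP_Fountain is an environment actor in the FortuneTeller area with continuously spinning Earth, Sun and Moon components.
; Each Tick it adds world yaw to the three scene components, scaled by world delta seconds for frame-rate independence.
; Each body turns at its own constant speed, with the Moon spinning opposite to the Earth and Sun.
; The construction script and other events are empty.
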(event `self.ReceiveTick`
  (params (DeltaSeconds :type "Float (single-precision)"))
  (`SceneComponent.K2_AddWorldRotation` (`self.EarthScene`) (`KismetMathLibrary.MakeRotator` 0.0 0.0 (* (`GameplayStatics.GetWorldDeltaSeconds`) 35.0)) false false)
  (`SceneComponent.K2_AddWorldRotation` (`self.SunScene`) (`KismetMathLibrary.MakeRotator` 0.0 0.0 (* (`GameplayStatics.GetWorldDeltaSeconds`) 30.0)) false false)
  (`SceneComponent.K2_AddWorldRotation` (`self.MoonScene`) (`KismetMathLibrary.MakeRotator` 0.0 0.0 (* (`GameplayStatics.GetWorldDeltaSeconds`) -25.0)) false false))

(fn `UserConstructionScript`)