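; BP_Wall_Spline is an environment actor for laying out walls along an editable spline.
; Unless IsDisabled is set, the construction script divides the spline into segments of Length times actor X scale, dropping any remainder.
; Each segment gets an X-forward spline mesh component with collision, using endpoint tangents clamped to segment length to follow the curve.
; The event graph contains no active logic.
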(fn `UserConstructionScript`
  (locals (ScaledLength :type "Float (double-precision)"))
  (bind _returnvalue_x (`KismetMathLibrary.BreakVector` (`self.GetActorScale3D`)))
  (if (not (`self.bIsDisabled`))
    (set `local.ScaledLength` (* _returnvalue_x (`self.Length`)))
    (for _index (range (`KismetMathLibrary.FTrunc` (/ (`SplineComponent.GetSplineLength` (`self.Spline`)) (`local.ScaledLength`))))
      (bind _returnvalue (`AddComponent|NODE_AddSplineMeshComponent-0`))
      (`SplineMeshComponent.SetForwardAxis` _returnvalue "X" true)
      (`PrimitiveComponent.SetCollisionEnabled` _returnvalue "QueryAndPhysics")
      (bind _returnvalue_2 (* _index (`local.ScaledLength`)))
      (bind _returnvalue_3 (* (+ _index 1) (`local.ScaledLength`)))
      (`SplineMeshComponent.SetStartAndEnd` _returnvalue (`SplineComponent.GetLocationAtDistanceAlongSpline` (`self.Spline`) _returnvalue_2 "Local") (`KismetMathLibrary.ClampVectorSize` (`SplineComponent.GetTangentAtDistanceAlongSpline` (`self.Spline`) _returnvalue_2 "Local") 0.0 (`local.ScaledLength`)) (`SplineComponent.GetLocationAtDistanceAlongSpline` (`self.Spline`) _returnvalue_3 "Local") (`KismetMathLibrary.ClampVectorSize` (`SplineComponent.GetTangentAtDistanceAlongSpline` (`self.Spline`) _returnvalue_3 "Local") 0.0 (`local.ScaledLength`)) true))))