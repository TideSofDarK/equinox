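; Examinable briefcase item with a three-cylinder combination lock puzzle that hides a pills pickup.
; Zooming into the lock enables cylinder clicks, each rotating a dial one step and checking its values against the solution.
; A match disables the lock, plays the opening animation and activates the pickup.
; Examining the pickup spawns the pills for the survival player controller and marks the briefcase empty, useless and discardable.
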(event `self.NumberLock.OnZoomed`
  (params (bIn :type Boolean))
  (set `InteractiveStaticMeshComponent.bCanBeClicked` bIn (`self.Cyl1`))
  (set `InteractiveStaticMeshComponent.bCanBeClicked` bIn (`self.Cyl2`))
  (set `InteractiveStaticMeshComponent.bCanBeClicked` bIn (`self.Cyl3`)))

(event `self.NumberLock.OnExamined`
  (`self.ZoomIntoExamineTarget_Event` (`self.NumberLock`)))

(event `self.Pickup.OnExamined`
  (bind _playercontrollersurvival (`/Game/FD10/Core/Survival/BPML_Shortcuts_Survival.GetSurvivalPlayerController`)
    (:`Success`
      (bind _returnvalue (`/Game/FD10/Core/BP_PlayerController_Survival.SpawnPickedItem` _playercontrollersurvival "/Game/FD10/Items/Pills/BP_PillsD.BP_PillsD_C"))
      (`self.PickupED` _returnvalue)
      (`ActorComponent.K2_DestroyComponent` (`self.PickupMesh`))
      (`ActorComponent.Deactivate` (`self.Pickup`))
      (set `/Game/FD10/Core/Survival/Items/BP_Item_Survival.bDiscardable` true (`self.Item`))
      (set `/Game/FD10/Core/Survival/Items/BP_Item_Survival.bUseless` true (`self.Item`))
      (set `/Game/FD10/Core/Survival/Items/BP_Item_Survival.Description` "Now it's empty." (`self.Item`))
      (`GameplayStatics.PlaySound2D` "/Game/FD10/Audio/UI/A_ItemPickup.A_ItemPickup" 1.0 1.0 0.0 null null))))

(event `self.Cyl1.OnClicked`
  (params (TouchedComponent :type "PrimitiveComponent Object Reference") (ButtonPressed :type "Key Structure"))
  (`self.RotateCylinder` TouchedComponent
    (:`Exec`
      (bind _bsolved (`self.CheckCode` :!label _label))
      (if _bsolved
        (`ActorComponent.Deactivate` (`self.NumberLock`))
        (`SkeletalMeshComponent.PlayAnimation` (`self.SkeletalMesh`) "/Game/FD10/Items/Briefcase/A_Open.A_Open" false)
        (`ActorComponent.Activate` (`self.Pickup`) false)
        (`self.ZoomIntoExamineTarget_Event` (`self.RootExamineTarget`) 1.0)))))

(event `self.Cyl2.OnClicked`
  (params (TouchedComponent :type "PrimitiveComponent Object Reference") (ButtonPressed :type "Key Structure"))
  (`self.RotateCylinder` TouchedComponent 1
    (:`Exec`
      (goto _label))))

(event `self.Cyl3.OnClicked`
  (params (TouchedComponent :type "PrimitiveComponent Object Reference") (ButtonPressed :type "Key Structure"))
  (`self.RotateCylinder` TouchedComponent 2
    (:`Exec`
      (goto _label))))

(fn `CheckCode`
  (returns (bSolved :type Boolean))
  (for (_array_element _array_index) (`self.Solution`)
    (if (not (== (`|GetArrayItem` (`self.Values`) _array_index) _array_element))
      (return false)))
  (return true))

(fn `UserConstructionScript`
  (`parent.UserConstructionScript`))