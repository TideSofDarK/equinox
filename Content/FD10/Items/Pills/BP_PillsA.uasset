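; BP_PillsA is a pill item that can be combined with BP_PillsD to produce BP_PillsMixed.
; Its Combine function checks the other item's class, spawns the mixed item through BP_SurvivalPlayerController, then destroys both source items.
; It plays the new item's CombineSound if valid and returns that item with a result enum, or a different result when the class does not match.
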(event `self.ReceiveBeginPlay`
  (`parent.ReceiveBeginPlay`))

(fn `Combine`
  (params (OtherItem :type "/Game/FD10/Core/Survival/Items/BP_SurvivalItem Object Reference"))
  (returns (Result :type "/Game/FD10/Core/Survival/Items/ECombineResult Enum") (NewItem :type "/Game/FD10/Core/Survival/Items/BP_SurvivalItem Object Reference"))
  (if (`KismetMathLibrary.ClassIsChildOf` (`GameplayStatics.GetObjectClass` OtherItem) "/Game/FD10/Items/Pills/BP_PillsD.BP_PillsD_C")
    (bind _returnvalue (`/Game/FD10/Core/Survival/BP_SurvivalPlayerController.SpawnPickedItem` (cast `/Game/FD10/Core/Survival/BP_SurvivalPlayerController` (`GameplayStatics.GetPlayerController` 0) :!pure true) "/Game/FD10/Items/Pills/BP_PillsMixed.BP_PillsMixed_C"))
    (`self.K2_DestroyActor` (`local.OtherItem`))
    (`self.K2_DestroyActor`)
    (bind _combinesound (`/Game/FD10/Core/Survival/Items/BP_SurvivalItem.CombineSound` _returnvalue))
    (`/Engine/EditorBlueprintResources/StandardMacros.IsValid` _combinesound
      (:`Is Valid`
        (`GameplayStatics.PlaySound2D` _combinesound 1.0 1.0 0.0 null null))
      (:`Is Not Valid`
        _))
    (return "NewEnumerator1" _returnvalue)
    (else
      (return "NewEnumerator2" null))))

(fn `UserConstructionScript`
  (`parent.UserConstructionScript`))