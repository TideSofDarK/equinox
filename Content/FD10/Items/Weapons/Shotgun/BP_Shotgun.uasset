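; BP_Shotgun is a shotgun weapon that extends a parent weapon class by overriding Fire and TraceShot.
; When the parent Fire succeeds, it plays the shot sound and spawns a Niagara muzzle flash at FireOrigin, then detaches it to stay in world space.
; TraceShot repeats the parent trace as randomized cone-spread pellets from FireOrigin, using its own fixed range and passing the full Damage to each.
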(fn `Fire`
  (returns (bSuccess :type Boolean))
  (bind _bsuccess (`parent.Fire`))
  (if _bsuccess
    (`GameplayStatics.PlaySoundAtLocation` "/Game/FD10/Items/Weapons/Shotgun/Audio/Fire/A_Shotgun_Fire_Cue.A_Shotgun_Fire_Cue" (`SceneComponent.K2_GetComponentLocation` (`self.FireOrigin`)) (struct) 1.0 1.0 0.0 null null null)
    (bind _returnvalue (`NiagaraFunctionLibrary.SpawnSystemAttached` "/Game/FD10/Items/Weapons/Sigismund/FX/NS_Sigismund_Flash.NS_Sigismund_Flash" (`self.FireOrigin`) "None" (2.5 0.0 0.0) (struct) "KeepRelativeOffset" true))
    (`SceneComponent.K2_DetachFromComponent` _returnvalue "KeepWorld" "KeepWorld" "KeepWorld" true)
    (return true)
    (else
      (return false))))

(fn `TraceShot`
  (params (Start :type "Vector Structure") (Direction :type "Vector Structure") (Length :type "Float (double-precision)") (Damage :type "Float (double-precision)"))
  (returns (bHit :type Boolean) (HitActor :type "Actor Object Reference"))
  (bind _fireorigin (`self.FireOrigin`))
  (for _ (range 5)
    (`parent.TraceShot` (`SceneComponent.K2_GetComponentLocation` _fireorigin) (+ (`SceneComponent.GetForwardVector` _fireorigin) (`KismetMathLibrary.RandomUnitVectorInConeInDegreesFromStream` (`SceneComponent.GetForwardVector` _fireorigin) 15.0 (`KismetMathLibrary.MakeRandomStream` (`KismetMathLibrary.RandomInteger` 1000)))) 1000.0 (`self.Damage`))))

(fn `UserConstructionScript`
  (`parent.UserConstructionScript`))