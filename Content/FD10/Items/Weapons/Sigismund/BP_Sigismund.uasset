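; Sigismund weapon Blueprint that adds firing audio and visual effects on top of its parent weapon class.
; Fire calls the parent and, only on success, plays the shot sound, spawns a muzzle flash and ejects a casing effect.
; The flash spawns attached to FireOrigin, then detaches to stay in world space.
; A separate event handles the delayed casing sound, since Fire is a function and cannot hold a Delay.
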(event `PlayBulletCasingSound_Event`
  (`KismetSystemLibrary.Delay` 0.75)
  (`GameplayStatics.PlaySoundAtLocation` "/Game/FD10/Items/Weapons/Sigismund/Audio/BulletCasing/A_Sigismund_BulletCasing_Cue.A_Sigismund_BulletCasing_Cue" (`self.K2_GetActorLocation`) (struct) 1.0 1.0 0.0 null null null))

(fn `Fire`
  (returns (bSuccess :type Boolean))
  (bind _bulletcasingorigin (`self.BulletCasingOrigin`))
  (bind _bsuccess (`parent.Fire`))
  (if _bsuccess
    (`GameplayStatics.PlaySoundAtLocation` "/Game/FD10/Items/Weapons/Sigismund/Audio/Fire/A_Sigismund_Fire_Cue.A_Sigismund_Fire_Cue" (`SceneComponent.K2_GetComponentLocation` (`self.FireOrigin`)) (struct) 1.0 1.0 0.0 null null null)
    (bind _returnvalue (`NiagaraFunctionLibrary.SpawnSystemAttached` "/Game/FD10/Items/Weapons/Sigismund/FX/NS_Sigismund_Flash.NS_Sigismund_Flash" (`self.FireOrigin`) "None" (2.5 0.0 0.0) (struct) "KeepRelativeOffset" true))
    (`SceneComponent.K2_DetachFromComponent` _returnvalue "KeepWorld" "KeepWorld" "KeepWorld" true)
    (`NiagaraFunctionLibrary.SpawnSystemAtLocation` "/Game/FD10/Items/Weapons/Sigismund/FX/NS_Sigismund_BulletCasing2.NS_Sigismund_BulletCasing2" (`SceneComponent.K2_GetComponentLocation` _bulletcasingorigin) (`SceneComponent.K2_GetComponentRotation` _bulletcasingorigin))
    (`self.PlayBulletCasingSound_Event`)
    (return true)
    (else
      (return false))))

(fn `UserConstructionScript`
  (`parent.UserConstructionScript`))