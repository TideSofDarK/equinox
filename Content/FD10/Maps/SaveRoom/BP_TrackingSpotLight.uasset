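; A spot light actor in the SaveRoom map folder that turns to follow the player.
; It caches the survival player pawn on BeginPlay.
; Each tick it eases its rotation toward a look-at rotation aimed at that pawn's location, using a linear blend scaled by frame delta for smoothed tracking.
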(event `self.ReceiveBeginPlay`
  (set `self.CachedCharacter` (`/Game/FD10/Core/Survival/BPFL_SurvivalUtilities.GetSurvivalPlayerPawn`)))

(event `self.ReceiveTick`
  (params (DeltaSeconds :type "Float (single-precision)"))
  (`self.K2_SetActorRotation` (`|EaseFunction` "Linear" (* DeltaSeconds 10.0) (`self.K2_GetActorRotation`) (`KismetMathLibrary.FindLookAtRotation` (`self.K2_GetActorLocation`) (`self.K2_GetActorLocation` (`self.CachedCharacter`))))))

(fn `UserConstructionScript`)